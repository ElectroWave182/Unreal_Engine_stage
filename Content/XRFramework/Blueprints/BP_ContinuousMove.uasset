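; BP_ContinuousMove drives continuous (smooth) locomotion for the player's BP_XRPawn in VR.
; Each Tick it offsets the cached pawn along the camera's yaw-only forward vector, scaled by MoveSpeed and summed Vector2DVar X and Y, without sweep or delta time.
; Two custom events toggle the pawn's TeleportActivated flag.
; While that flag is set, movement is replaced by a French debug message.
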(event `self.ReceiveTick`
  (params (DeltaSeconds :type "Float (single-precision)"))
  (bind _bp_xrpawnvar (`self.BP_XRPawnVar`))
  (bind (_x _y) (`KismetMathLibrary.BreakVector2D` (`/Game/XRFramework/Blueprints/BP_XRPawn.Vector2DVar` _bp_xrpawnvar)))
  (if (`/Game/XRFramework/Blueprints/BP_XRPawn.TeleportActivated` (`self.BP_XRPawnVar`))
    (`KismetSystemLibrary.PrintString` "Tu peux plus bouger normalement mon p'tit gars ! TP activée !" true true (struct :`R` 1.0 :`B` 0.057586 :`A` 1.0) 5.0)
    (else
      (bind _output_get (set `self.FowardCamVar` (`KismetMathLibrary.GetForwardVector` (`KismetMathLibrary.MakeRotator` 0.0 0.0 (.yaw (`SceneComponent.K2_GetComponentRotation` (`/Game/XRFramework/Blueprints/BP_XRPawn.Camera` _bp_xrpawnvar)))))))
      (`self.K2_SetActorLocation` (`self.BP_XRPawnVar`) (+ (* (* _output_get (`self.MoveSpeed`)) (+ _x _y)) (`self.K2_GetActorLocation` _bp_xrpawnvar)) false false))))

(event `self.ReceiveBeginPlay`
  (bind _asbp_xrpawn (cast `/Game/XRFramework/Blueprints/BP_XRPawn` (`GameplayStatics.GetPlayerPawn` 0)))
  (set `self.BP_XRPawnVar` _asbp_xrpawn))

(event `DisableContinuousMoveEvent`
  (set `/Game/XRFramework/Blueprints/BP_XRPawn.TeleportActivated` true (`self.BP_XRPawnVar`)))

(event `ContinuousMoveEvent`
  (set `/Game/XRFramework/Blueprints/BP_XRPawn.TeleportActivated` false (`self.BP_XRPawnVar`)))

(fn `UserConstructionScript`)