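; BP_Maillet is a grabbable mallet actor for the XR framework.
; On grab, its grab component events enable player input, add the left or right weapon Enhanced Input mapping context for the holding hand, and hide that hand's message through the motion controller's owner.
; On drop, they disable input, remove the context and show the message again.
; The Blueprint itself contains no strike or input action logic.
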(event `self.BP_GrabComponent.OnGrabbed`
  (bind _bp_grabcomponent (`self.BP_GrabComponent`))
  (bind _returnvalue (`|EnumEquality` (`/Game/XRFramework/Blueprints/BP_GrabComponent.GetHeldByHand` _bp_grabcomponent) "Right"))
  (`self.EnableInput` (`GameplayStatics.GetPlayerController` 0))
  (message `/Game/XRFramework/Blueprints/BPI_PawnAnim.HideUnhideHand` (`ActorComponent.GetOwner` (`/Game/XRFramework/Blueprints/BP_GrabComponent.MotionControllerRef` _bp_grabcomponent)) true _returnvalue)
  (`EnhancedInputSubsystemInterface.AddMappingContext` (pcsubsystem `EnhancedInputLocalPlayerSubsystem` (`GameplayStatics.GetPlayerController` 0)) (select `bool` _returnvalue :`false` "/Game/XRFramework/Input/IMC_Weapon_Left.IMC_Weapon_Left" :`true` "/Game/XRFramework/Input/IMC_Weapon_Right.IMC_Weapon_Right" :!type "InputMappingContext Object Reference") 1 (struct)))

(event `self.BP_GrabComponent.OnDropped`
  (bind _bp_grabcomponent (`self.BP_GrabComponent`))
  (bind _returnvalue (`|EnumEquality` (`/Game/XRFramework/Blueprints/BP_GrabComponent.GetHeldByHand` _bp_grabcomponent) "Right"))
  (`self.DisableInput` (`GameplayStatics.GetPlayerController` 0))
  (message `/Game/XRFramework/Blueprints/BPI_PawnAnim.HideUnhideHand` (`ActorComponent.GetOwner` (`/Game/XRFramework/Blueprints/BP_GrabComponent.MotionControllerRef` _bp_grabcomponent)) false _returnvalue)
  (`EnhancedInputSubsystemInterface.RemoveMappingContext` (pcsubsystem `EnhancedInputLocalPlayerSubsystem` (`GameplayStatics.GetPlayerController` 0)) (select `bool` _returnvalue :`false` "/Game/XRFramework/Input/IMC_Weapon_Left.IMC_Weapon_Left" :`true` "/Game/XRFramework/Input/IMC_Weapon_Right.IMC_Weapon_Right" :!type "InputMappingContext Object Reference") (struct)))

(fn `UserConstructionScript`)