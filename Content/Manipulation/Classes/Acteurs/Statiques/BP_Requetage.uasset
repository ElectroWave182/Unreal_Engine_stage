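; Actor that handles external data requests for the robot digital-twin software: Onshape CAD import and communication with real robots.
; An HTTP call to the Onshape API maps part names to the selected assembly, then rebuilds joints with axes, constraints and limits, spawning debug indicators.
; On BeginPlay it launches Node-RED and exchanges robot name, sensor information and placements with it through project JSON files, detecting motion from file changes or Universal Robots speed scaling.
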(event `self.ReceiveBeginPlay`
  ; Mise en place
  (`self.robotConnecter` null)
  (`self.placementsLire`)
  (`self.communicationLancer`))

(event `api`
  (params (lien :type String))
  (bind (_adresserequete _parametresrequete) (`self.apiAdresse` lien))
  ; API Onshape : importe les liaisons depuis un document en ligne
  (bind (_outheader _result_body) (`|HttpRequest` _adresserequete "Get" _parametresrequete)
    (:`On Success`
      (bind _outjsonobject (`JsonBlueprintFunctionLibrary.FromString` _result_body))
      (`self.apiDonneesRecuperer` _outjsonobject))))

(fn `aBougeUniversalRobots`
  (returns (aBouge :type Boolean))
  (locals (champMode :type String :default "robotModeData") (champVitesse :type String :default "speedScaling"))
  ; {robotModeData {speedScaling}} == 1
  (bind _outjsonobject (`JsonBlueprintFunctionLibrary.FromString` (`.informations` (`self.informationsObtenir`))))
  (bind _outvalue (`|GetJsonField` _outjsonobject (`local.champMode`)))
  (bind _outvalue_2 (`|GetJsonField` _outvalue (`local.champVitesse`)))
  (return (== _outvalue_2 1)))

(fn `apiAdresse`
  (params (adresseDocument :type String :default "https://cad.onshape.com/documents/2b469794bb6dce26d46feb15/w/1572c4b1f21e33ff5c33d7bd/e/bb07d9e351da00cbe9a8bb39"))
  (returns (adresseRequete :type String) (parametresRequete :type "HttpHeader Structure"))
  (locals (proprietes :type "HttpHeader Structure") (adresseAPI :type String :default "https://cad.onshape.com/api/v14/assemblies/d/") (categorieDocument :type String :default "documents") (categorieElement :type String :default "e") (categorieWorkspace :type String :default "w") (enTete :type String :default "Authorization") (valeurCle :type String :default "Basic b25fanYwVG1wOG0xaVJNRHBDUE1waEZtOmd4UGtLNXNOVFcyMU5IQ1IxZ2RadHVMV1V6QTM0ajRqdmxjU0p5ZzVyUFhJdjdkcw=="))
  (bind (_contenu _reste) (`/Game/Manipulation/Classes/Abstraites/BPFL_Caracteres.balise` (`local.adresseDocument`) (`local.categorieDocument`)))
  (bind (_contenu_2 _reste_2) (`/Game/Manipulation/Classes/Abstraites/BPFL_Caracteres.balise` _reste (`local.categorieWorkspace`)))
  (`|ExecutionSequence`
    (:`then_0`
      ; On indique une clé de cryptage
      (bind _output_get (set `local.proprietes` (`|MakeRequestHeader` "Json")))
      (`HttpBlueprintFunctionLibrary.AddHeader` _output_get (`local.enTete`) (`local.valeurCle`)))
    (:`then_1`
      ; On met en forme l'adresse de la requête "Get assemblies"
      (return (`KismetStringLibrary.Concat_StrStr` (`local.adresseAPI`) _contenu "/" (`local.categorieWorkspace`) "/" _contenu_2 "/" (`local.categorieElement`) "/" (`/Game/Manipulation/Classes/Abstraites/BPFL_Caracteres.balise` _reste_2 (`local.categorieElement`)) "?" (`self.apiParametres`)) (`local.proprietes`)))))

(fn `apiDonneesRecuperer`
  (params (onshape :type "JsonObjectWrapper Structure"))
  (locals (liaisonType :type String) (identifiantsLies :type "Array of String") (champAssemblage :type String :default "rootAssembly") (champChemin :type String :default "path") (champLiaisonDonnees :type String :default "featureData") (champLiaisons :type String :default "features") (champLiaisonType :type String :default "mateType") (champLie :type String :default "matedOccurrence") (champLies :type String :default "matedEntities") (champMatriceTransformation :type String :default "matedCS") (champOrigine :type String :default "origin") (champPieces :type String :default "occurrences") (champPlacement :type String :default "transform") (champSousAssemblages :type String :default "subAssemblies"))
  (bind _returnvalue (`GameplayStatics.GetActorOfClass` "/Game/Manipulation/Classes/Acteurs/Statiques/BP_Logiciel.BP_Logiciel_C"))
  (`/Engine/EditorBlueprintResources/StandardMacros.IsValid` (`/Game/Manipulation/Classes/Acteurs/Statiques/BP_Logiciel.assemblageSelectionne` _returnvalue)
    (:`Is Valid`
      (`|ExecutionSequence`
        (:`then_0`
          (`BlueprintMapLibrary.Map_Clear` (`self.piecesNom`)))
        (:`then_1`
          ; On parcourt les champs Json utiles : subAssemblies [{}], rootAssembly {}
          (bind _outvalue (`|GetJsonField` (`local.onshape`) (`local.champAssemblage`)))
          (bind _outvalue_2 (`|GetJsonField` (`local.onshape`) (`local.champSousAssemblages`)))
          (for _array_element _outvalue_2
            (`self.apiMetadonneesRecuperer` _array_element)
            (`self.apiLiaisonsRecuperer` _array_element))
          (`self.apiMetadonneesRecuperer` _outvalue)
          (`self.apiLiaisonsRecuperer` _outvalue))))))

(fn `apiDonneesTraiter`
  (params (matriceOnshape :type "JsonObjectWrapper Structure") (origine :type "Array of Float (double-precision)") (limitesOnshape :type "Map of String to Float (double-precision)") (liaisonType :type String) (identifiantsLies :type "Array of String"))
  (locals (axeLie :type "/Game/Manipulation/Enumérateurs/E_Axe Enum" :default "NewEnumerator3") (cadres :type "Set of EConstraintFrame Enum") (transformationLiee :type "/Game/Manipulation/Enumérateurs/E_Transformation Enum" :default "NewEnumerator0") (contraintes :type "Map of /Game/Manipulation/Enumérateurs/E_Transformation Enum to /Game/Manipulation/Types/S_ContraintesAxes Structure") (listeCoordonnees :type "Array of Float (double-precision)") (robotLie :type "/Game/Manipulation/Classes/Acteurs/BP_Robot Object Reference") (rotation :type "Rotator Structure") (rotationCadre :type "Rotator Structure") (pieceLieeA :type "StaticMeshComponent Object Reference") (pieceLieeB :type "StaticMeshComponent Object Reference") (champAxeX :type String :default "xAxis") (champAxeY :type String :default "yAxis") (champAxeZ :type String :default "zAxis") (translation :type "Vector Structure") (translationCadre :type "Vector Structure"))
  (bind _matriceonshape (`local.matriceOnshape`))
  (bind _identifiantslies (`local.identifiantsLies`))
  (bind _listecoordonnees (`local.listeCoordonnees`))
  (bind (_trouvee _amplitude _milieu) (`/Game/Manipulation/Classes/Abstraites/BPFL_Contrainte.limiteOnshape` (`local.limitesOnshape`) (`local.transformationLiee`) (`local.axeLie`)))
  (bind (_assemblage _piece) (`self.apiPieceObtenir` (`|GetArrayItem` _identifiantslies)))
  (`|ExecutionSequence`
    (:`then_0`
      (set `local.translation` (`/Game/Manipulation/Classes/Abstraites/BPFL_Vecteur.onshapeVersVecteur` (`local.origine`))))
    (:`then_1`
      ; On reconstruit la rotation à partir de la matrice d'Onshape
      (bind _outvalue (`|GetJsonField` _matriceonshape (`local.champAxeX`)))
      (set `local.listeCoordonnees` _outvalue))
    (:`then_2`
      (bind _outvalue_2 (`|GetJsonField` _matriceonshape (`local.champAxeY`)))
      (`KismetArrayLibrary.Array_Append` (`local.listeCoordonnees`) _outvalue_2))
    (:`then_3`
      (bind _outvalue_3 (`|GetJsonField` _matriceonshape (`local.champAxeZ`)))
      (`KismetArrayLibrary.Array_Append` _listecoordonnees _outvalue_3)
      (set `local.rotation` (`/Game/Manipulation/Classes/Abstraites/BPFL_Rotation.onshapeVersRotation` _listecoordonnees)))
    (:`then_4`
      ; On retrouve les pièces correspondantes grâce à l'identifiant
      (set `local.robotLie` _assemblage)
      (set `local.pieceLieeA` _piece)
      (set `local.pieceLieeB` (`.piece` (`self.apiPieceObtenir` (`|GetArrayItem` _identifiantslies 1)))))
    (:`then_5`
      (`/Engine/EditorBlueprintResources/StandardMacros.IsValid` (`local.pieceLieeA`)
        (:`Is Valid`
          (`/Engine/EditorBlueprintResources/StandardMacros.IsValid` (`local.pieceLieeB`)
            (:`Is Valid`
              (`|ExecutionSequence`
                (:`then_0`
                  (`/Game/Manipulation/Classes/Acteurs/BP_GrapheLiaisons.liaisonCreer` (`/Game/Manipulation/Classes/Acteurs/BP_Robot.liaisons` (`local.robotLie`)) (`local.pieceLieeA`) (`local.pieceLieeB`)))
                (:`then_1`
                  ; On part d'abord de contraintes bloquantes ou libres
                  (set `local.contraintes` (`/Game/Manipulation/Classes/Abstraites/BPFL_Contrainte.liaisonOnshape` (`local.liaisonType`))))
                (:`then_2`
                  (bind _etat (`/Game/Manipulation/Classes/Abstraites/BPML_Contrainte.pourChaqueEtat` (`local.contraintes`))
                    (:`boucle`
                      ; Pour chaque limite fournie par Onshape, on applique une amplitude directement sur l'attribut prévu par le composant
                      (set `local.transformationLiee` (break `/Game/Manipulation/Types/S_Contrainte` _etat))
                      (set `local.axeLie` (`.axe_7_BF3857B14A3C2C2C5F9E5E99CA4A2D8B` (break `/Game/Manipulation/Types/S_Contrainte` _etat)))
                      (if _trouvee
                        (`/Game/Manipulation/Classes/Abstraites/BPFL_Contrainte.etatPhysiqueDefinir` (`local.contraintes`) (make `/Game/Manipulation/Types/S_Contrainte` (`local.transformationLiee`) (`local.axeLie`) (make `/Game/Manipulation/Types/S_Physique` "NewEnumerator1" _amplitude _milieu)))))))
                (:`then_3`
                  ; On met à jour tous les degrés de liberté de la contrainte physique de la pièce
                  (`/Game/Manipulation/Classes/Acteurs/BP_Robot.liaisonChanger` (`local.robotLie`) (make `/Game/Manipulation/Types/S_Liaison` (`/Game/Manipulation/Classes/Abstraites/BPFL_Transformation.transformationVersPlacement` (`KismetMathLibrary.MakeTransform` (`local.translation`) (`local.rotation`))) (`local.contraintes`)) (`local.pieceLieeA`) (`local.pieceLieeB`) "NewEnumerator2" "NewEnumerator4")
                  ;[0.08185 0.3237 0.9479 0.5] Relier au changement de liaison pour la visualiser et ainsi débugguer
                  (`|SpawnActorFromClass` "/Game/Manipulation/Classes/Acteurs/BP_Indicateur.BP_Indicateur_C" (`SceneComponent.K2_GetComponentToWorld` (`/Game/Manipulation/Classes/Acteurs/BP_GrapheLiaisons.composantObtenir` (`/Game/Manipulation/Classes/Acteurs/BP_Robot.liaisons` (`local.robotLie`)) (`local.pieceLieeA`) (`local.pieceLieeB`))) "Undefined" "MultiplyWithRoot" null null))))))))))

(fn `apiLiaisonsRecuperer`
  (params (onshapeAssemblage :type "JsonObjectWrapper Structure"))
  (locals (identifiantsLies :type "Array of String") (liaisonType :type String) (limites :type "Map of String to Float (double-precision)") (champAssemblage :type String :default "rootAssembly") (champChemin :type String :default "path") (champLiaisonDonnees :type String :default "featureData") (champLiaisons :type String :default "features") (champLiaisonType :type String :default "mateType") (champLie :type String :default "matedOccurrence") (champLies :type String :default "matedEntities") (champLimites :type String :default "mateLimits") (champMatriceTransformation :type String :default "matedCS") (champOrigine :type String :default "origin") (champPieces :type String :default "occurrences") (champPlacement :type String :default "transform") (champSousAssemblages :type String :default "subAssemblies"))
  (bind _champlies (`local.champLies`))
  ; On parcourt les champs Json voulus pour les liaisons : features [{featureData {matedEntities [{matedOccurence [*]}], matedCS {xAxis [*], yAxis [*], zAxis [*], origin [*]}, mateLimits {}, mateType}}]
  (bind _outvalue (`|GetJsonField` onshapeAssemblage (`local.champLiaisons`)))
  (for _array_element _outvalue
    (bind _outvalue_2 (`|GetJsonField` _array_element (`local.champLiaisonDonnees`)))
    (bind _outvalue_3 (`|GetJsonField` _outvalue_2 (`local.champLiaisonType`)))
    (set `local.liaisonType` _outvalue_3)
    (bind _outvalue_4 (`|GetJsonField` _outvalue_2 (`local.champLimites`)))
    (set `local.limites` _outvalue_4)
    (`KismetArrayLibrary.Array_Clear` (`local.identifiantsLies`))
    (bind _returnvalue (`JsonBlueprintFunctionLibrary.HasField` _outvalue_2 _champlies))
    (if _returnvalue
      (bind _outvalue_5 (`|GetJsonField` _outvalue_2 _champlies))
      (for _array_element_2 _outvalue_5
        (bind _outvalue_6 (`|GetJsonField` _array_element_2 (`local.champLie`)))
        (`KismetArrayLibrary.Array_Add` (`local.identifiantsLies`) (`|GetArrayItem` _outvalue_6 (`KismetArrayLibrary.Array_LastIndex` _outvalue_6))))
      (if (not (`KismetArrayLibrary.Array_Contains` (`local.identifiantsLies`)))
        (`|ExecutionSequence`
          (:`then_0`
            (bind _outvalue_7 (`|GetJsonField` (`|GetArrayItem` _outvalue_5) (`local.champMatriceTransformation`))))
          (:`then_1`
            (bind _outvalue_8 (`|GetJsonField` (`|GetArrayItem` _outvalue_5 1) (`local.champMatriceTransformation`)))
            (bind _outvalue_9 (`|GetJsonField` _outvalue_8 (`local.champOrigine`)))
            (`self.apiDonneesTraiter` _outvalue_7 _outvalue_9 (`local.limites`) (`local.liaisonType`) (`local.identifiantsLies`))))))))

(fn `apiMetadonneesRecuperer`
  (params (onshapeAssemblage :type "JsonObjectWrapper Structure"))
  (locals (champIdentifiant :type String :default "id") (champMetadonnees :type String :default "instances") (champNom :type String :default "name") (champType :type String :default "type") (champTypePiece :type String :default "Part"))
  ; On vient chercher les noms des pièces Onshape pour les identifier aux pièces de notre logiciel : ... {instances [{id, type, name}]}
  (bind _outvalue (`|GetJsonField` onshapeAssemblage (`local.champMetadonnees`)))
  (for _array_element _outvalue
    (bind _outvalue_2 (`|GetJsonField` _array_element (`local.champType`)))
    (if (`KismetStringLibrary.EqualEqual_StrStr` _outvalue_2 (`local.champTypePiece`))
      (bind _outvalue_3 (`|GetJsonField` _array_element (`local.champNom`)))
      (bind _outvalue_4 (`|GetJsonField` _array_element (`local.champIdentifiant`)))
      (`BlueprintMapLibrary.Map_Add` (`self.piecesNom`) _outvalue_4 _outvalue_3))))

(fn `apiParametres`
  (returns (concatenationParametres :type String))
  (locals (concatenation :type String) (concatenationPrecedente :type String) (separateur :type String :default "&") (parametres :type "Map of String to Boolean"))
  (bind (_keypin _valuepin) (`|MapForEach` (`local.parametres`))
    (:`then`
      ; On concatène les paramètres et leurs valeurs uns à uns, en prenant soin d'ignorer le dernier séparateur
      (bind _output_get (set `local.concatenationPrecedente` (`KismetStringLibrary.Concat_StrStr` (`local.concatenation`) _keypin (`KismetStringLibrary.Conv_BoolToString` _valuepin))))
      (set `local.concatenation` (`KismetStringLibrary.Concat_StrStr` _output_get (`local.separateur`))))
    (:`CompletedPin`
      (return (`local.concatenationPrecedente`)))))

(fn `apiPieceObtenir`
  (params (identifiant :type String))
  (returns (assemblage :type "/Game/Manipulation/Classes/Acteurs/BP_Robot Object Reference") (piece :type "StaticMeshComponent Object Reference"))
  ; On va chercher la pièce à partir de l'identifiant fourni
  (bind _returnvalue (`GameplayStatics.GetActorOfClass` "/Game/Manipulation/Classes/Acteurs/Statiques/BP_Logiciel.BP_Logiciel_C"))
  (bind _assemblage (`/Game/Manipulation/Classes/Acteurs/Statiques/BP_Logiciel.assemblageSelectionne` _returnvalue))
  (bind _crochets (`/Game/Manipulation/Classes/Abstraites/BPFL_Piece.nomOnshape` _assemblage (`BlueprintMapLibrary.Map_Find` (`self.piecesNom`) identifiant)))
  (bind (_reussite _piece) (`/Game/Manipulation/Classes/Acteurs/BP_Robot.pieceObtenir` _assemblage _crochets))
  (if _reussite
    (return _assemblage _piece)
    (else
      (`/Game/Manipulation/Classes/Abstraites/BPFL_Caracteres.erreurAfficher` (`|FormatText` "la pièce {pièce}, demandée par Onshape, n'a pas encore été importée" _crochets)))))

(fn `communicationLancer`
  (`|ExecutionSequence`
    (:`then_0`
      ; On réinitialise les informations reçues du robot
      (bind _outjsonobject (`JsonBlueprintFunctionLibrary.FromFile` (make `FilePath` "")))
      (`JsonBlueprintFunctionLibrary.ToFile` _outjsonobject (make `FilePath` (`self.fichierInformations`))))
    (:`then_1`
      ; Lancement de la communication avec les robots
      (bind _returnvalue (`Systeme.executer` (`self.fichierNodeRed`) "" true))
      (bind _output_get (set `self.nodeRed` _returnvalue))
      (if (not _output_get)
        ; Erreur : la commande "node-red" a échoué
        (`/Game/Manipulation/Classes/Abstraites/BPFL_Caracteres.erreurAfficher` "installation de Node-RED incorrecte")))))

(fn `fichierAttributsConnexion`
  (returns (cheminAbsolu :type String))
  (locals (cheminRelatif :type String :default "node-red/attributs.json"))
  ; Chemin vers le nom du robot connecté
  (return (`KismetStringLibrary.Concat_StrStr` (`KismetSystemLibrary.GetProjectDirectory`) (`local.cheminRelatif`))))

(fn `fichierInformations`
  (returns (cheminAbsolu :type String))
  (locals (cheminRelatif :type String :default "node-red/informations.json"))
  ; Chemin vers les informations captées par le robot
  (return (`KismetStringLibrary.Concat_StrStr` (`KismetSystemLibrary.GetProjectDirectory`) (`local.cheminRelatif`))))

(fn `fichierNodeRed`
  (returns (cheminAbsolu :type String))
  (locals (cheminRelatif :type String :default "node-red/lancement.bat"))
  ; Chemin vers le lanceur du gestionnaire de communication Node-RED
  (return (`KismetStringLibrary.Concat_StrStr` (`KismetSystemLibrary.GetProjectDirectory`) (`local.cheminRelatif`))))

(fn `fichierPlacementJumeau`
  (returns (cheminAbsolu :type String))
  (locals (cheminRelatif :type String :default "node-red/placementJumeau.json"))
  ; Chemin vers les informations captées par le robot
  (return (`KismetStringLibrary.Concat_StrStr` (`KismetSystemLibrary.GetProjectDirectory`) (`local.cheminRelatif`))))

(fn `fichierPlacementReel`
  (returns (cheminAbsolu :type String))
  (locals (cheminRelatif :type String :default "node-red/placementReel.json"))
  ; Chemin vers les informations captées par le robot
  (return (`KismetStringLibrary.Concat_StrStr` (`KismetSystemLibrary.GetProjectDirectory`) (`local.cheminRelatif`))))

(fn `fichierRobotConnecte`
  (returns (cheminAbsolu :type String))
  (locals (cheminRelatif :type String :default "node-red/robotConnecte.json"))
  ; Chemin vers le nom du robot connecté
  (return (`KismetStringLibrary.Concat_StrStr` (`KismetSystemLibrary.GetProjectDirectory`) (`local.cheminRelatif`))))

(fn `informationsObtenir`
  (returns (connexion :type "/Game/Manipulation/Enumérateurs/E_ConnexionStatut Enum") (informations :type String) (robotConnecte :type String))
  (locals (champNomRobot :type String :default "nom") (nomRobot :type String))
  (bind _nomrobot (`local.nomRobot`))
  ; On lit le nom du robot connecté
  (bind _outjsonobject (`JsonBlueprintFunctionLibrary.FromFile` (make `FilePath` (`self.fichierRobotConnecte`))))
  (bind _outvalue (`|GetJsonField` _outjsonobject (`local.champNomRobot`)))
  (bind _output_get (set `local.nomRobot` _outvalue))
  ; On considère qu'il n'y a pas de transit d'informations si l'on a pas spécifié de robot auquel se connecter
  (if (`KismetStringLibrary.IsEmpty` _output_get)
    (return "NewEnumerator0" "" "")
    (else
      ; On vérifie qu'il y ait bien une récupération en cours sur le réseau
      (if (and (`self.capteurs`) (`self.nodeRed`))
        ; Et l'on va chercher les informations du robot dans le fichier
        (bind _outjsonobject_2 (`JsonBlueprintFunctionLibrary.FromFile` (make `FilePath` (`self.fichierInformations`))))
        (bind _outvalue_2 (`|GetJsonField` _outjsonobject_2 _nomrobot))
        (bind _outjsonstring (`|StructToJsonString` _outvalue_2))
        (return (select `bool` (`/Game/Manipulation/Classes/Abstraites/BPFL_Caracteres.jsonEstVide` _outvalue_2) :`false` "NewEnumerator1" :`true` "NewEnumerator3" :!type "/Game/Manipulation/Enumérateurs/E_ConnexionStatut Enum") _outjsonstring _nomrobot)
        (else
          (return "NewEnumerator2" "" (`local.nomRobot`)))))))

(fn `placementsEcrire`
  (params (decalages :type "Array of Float (double-precision)"))
  (locals (champDecalages :type String :default "decalages") (contenu :type "JsonObjectWrapper Structure"))
  (bind _outjsonobject (`JsonBlueprintFunctionLibrary.FromFile` (make `FilePath` (`self.fichierPlacementJumeau`))))
  (bind _output_get (set `local.contenu` _outjsonobject))
  (`|SetJsonField` _output_get (`local.champDecalages`) decalages)
  (`JsonBlueprintFunctionLibrary.ToFile` (`local.contenu`) (make `FilePath` (`self.fichierPlacementJumeau`))))

(fn `placementsLire`
  (returns (decalages :type "Array of Float (double-precision)") (aBouge :type Boolean))
  (locals (champDecalages :type String :default "decalages") (contenuDifferent :type Boolean))
  ; En plus de lire le fichier, on regarde s'il a changé depuis la dernière lecture
  (bind _outjsonobject (`JsonBlueprintFunctionLibrary.FromFile` (make `FilePath` (`self.fichierPlacementReel`))))
  (bind _outjsonstring (`|StructToJsonString` _outjsonobject))
  (set `local.contenuDifferent` (`KismetStringLibrary.NotEqual_StrStr` _outjsonstring (`self.contenuPlacementReel`)))
  (set `self.contenuPlacementReel` _outjsonstring)
  (bind _outvalue (`|GetJsonField` _outjsonobject (`local.champDecalages`)))
  (return _outvalue (or (`local.contenuDifferent`) (`self.aBougeUniversalRobots`))))

(fn `rafraichissementInitialiser`
  (locals (champRafraichissement :type String :default "rafraichissement") (periode :type "Float (double-precision)" :default 1.0))
  ; Temps entre deux prises d'informations sur le robot
  (bind _outjsonobject (`JsonBlueprintFunctionLibrary.FromFile` (make `FilePath` (`self.fichierAttributsConnexion`))))
  (`|SetJsonField` _outjsonobject (`local.champRafraichissement`) (`local.periode`))
  (`JsonBlueprintFunctionLibrary.ToFile` _outjsonobject (make `FilePath` (`self.fichierAttributsConnexion`))))

(fn `robotConnecter`
  (params (robot :type "/Game/Manipulation/Classes/Acteurs/BP_Robot Object Reference"))
  (locals (champAdresse :type String :default "adresse") (champNom :type String :default "nom") (robotConnecte :type "JsonObjectWrapper Structure") (ancienneAdresse :type String) (nomRobot :type String))
  (bind _robot (`local.robot`))
  ; Si Node-RED a été lancé, on se connecte au véritable robot
  (`|ExecutionSequence`
    (:`then_0`
      (`/Engine/EditorBlueprintResources/StandardMacros.IsValid` _robot
        (:`Is Valid`
          (set `local.nomRobot` (`/Game/Manipulation/Classes/Acteurs/BP_Robot.nomObtenir` _robot)))))
    (:`then_1`
      (bind _outjsonobject (`JsonBlueprintFunctionLibrary.FromFile` (make `FilePath` (`self.fichierRobotConnecte`))))
      (`|SetJsonField` _outjsonobject (`local.champNom`) (`local.nomRobot`))
      (`JsonBlueprintFunctionLibrary.ToFile` _outjsonobject (make `FilePath` (`self.fichierRobotConnecte`))))))

(fn `UserConstructionScript`)