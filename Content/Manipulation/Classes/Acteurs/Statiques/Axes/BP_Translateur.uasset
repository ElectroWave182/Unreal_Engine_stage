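; BP_Translateur is a translation gizmo that drags a piece or assembly along its X, Y or Z arrow, extending a parent axis class.
; Anchoring stores the organ's start position, cursor hit point and chosen actor axis.
; While pulled, it finds the closest point between mouse ray and axis line, then moves the organ with sweep and itself with it.
; LierStop passes the used axis to the assembly to update the link between two pieces.
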(fn `ancrageChanger`
  (params (organeAncre :type "SceneComponent Object Reference"))
  ; On retient la position de départ de l'organe pour pouvoir la comparer ensuite
  (`parent.ancrageChanger` organeAncre)
  (switch `/Game/Manipulation/Enumérateurs/E_Axe` (`self.axeUtilise`)
    (:`NewEnumerator0`
      _)
    (:`NewEnumerator1`
      _)
    (:`NewEnumerator2`
      _)
    (:`NewEnumerator4`
      _))
  (set `self.departOrgane` (`SceneComponent.K2_GetComponentLocation` organeAncre))
  (`|ExecutionSequence`
    (:`then_0`
      ; Position de départ du curseur
      (bind _returnvalue (`GameplayStatics.GetActorOfClass` "/Game/Manipulation/Classes/Acteurs/Statiques/BP_Personnage.BP_Personnage_C"))
      (set `self.departTirage` (`/Game/Manipulation/Classes/Acteurs/Statiques/BP_Personnage.curseurCollision` _returnvalue "TraceTypeQuery3")))
    (:`then_1`
      ; Axe de déplacement
      (set `self.direction` (select `/Game/Manipulation/Enumérateurs/E_Axe` (`self.axeUtilise`) :`NewEnumerator0` (`self.GetActorForwardVector`) :`NewEnumerator1` (`self.GetActorRightVector`) :`NewEnumerator2` (`self.GetActorUpVector`))))))

(fn `axesInitialiser`
  (`parent.axesInitialiser`)
  (`|ExecutionSequence`
    (:`then_0`
      (`BlueprintMapLibrary.Map_Add` (`self.axes`) (`self.flecheX`) "NewEnumerator0"))
    (:`then_1`
      (`BlueprintMapLibrary.Map_Add` (`self.axes`) (`self.flecheY`) "NewEnumerator1"))
    (:`then_2`
      (`BlueprintMapLibrary.Map_Add` (`self.axes`) (`self.flecheZ`) "NewEnumerator2"))))

(fn `lierStop`
  (returns (assemblage :type "/Game/Manipulation/Classes/Acteurs/BP_Robot Object Reference") (pieceA :type "StaticMeshComponent Object Reference") (pieceB :type "StaticMeshComponent Object Reference"))
  (bind _axeutilise (`self.axeUtilise`))
  ; Prise en compte des paramètres : l'axe (x, y, z) et l'état de la contrainte (libre, limitée ou bloquée)
  (bind (_assemblage _piecea _pieceb) (`parent.lierStop`))
  (`/Engine/EditorBlueprintResources/StandardMacros.IsValid` _assemblage
    (:`Is Valid`
      (`|ExecutionSequence`
        (:`then_0`
          (switch `/Game/Manipulation/Enumérateurs/E_Axe` _axeutilise
            (:`NewEnumerator0`
              _)
            (:`NewEnumerator1`
              _)
            (:`NewEnumerator2`
              _)
            (:`NewEnumerator4`
              _))
          (`/Game/Manipulation/Classes/Acteurs/BP_Robot.liaisonChanger` :`self` _assemblage :`pieceA` _piecea :`pieceB` _pieceb :`axe` _axeutilise))
        (:`then_1`
          (return _assemblage _piecea _pieceb))))))

(fn `organeDeplacement`
  (params (direction :type "Vector Structure" :default (1.0 0.0 0.0)))
  (returns (position :type "Vector Structure"))
  ; On cherche le point le plus proche de la demi-droite du pointeur souris
  (bind _returnvalue (`GameplayStatics.GetActorOfClass` "/Game/Manipulation/Classes/Acteurs/Statiques/BP_Personnage.BP_Personnage_C"))
  (bind (_position _direction) (`/Game/Manipulation/Classes/Acteurs/Statiques/BP_Personnage.curseurPlacement` _returnvalue))
  ; On retranscrit ce déplacement sur la pièce
  (return (+ (- (`.pointD2` (`/Game/Manipulation/Classes/Abstraites/BPFL_Vecteur.proximiteDroites` _position (`self.departTirage`) _direction (`local.direction`))) (`self.departTirage`)) (`self.departOrgane`))))

(fn `tirer`
  (returns (organe :type "SceneComponent Object Reference") (axe :type "/Game/Manipulation/Enumérateurs/E_Axe Enum"))
  (locals (cible :type "SceneComponent Object Reference") (positionFin :type "Vector Structure"))
  (bind _positionfin (`local.positionFin`))
  ; On tire sur un des trois axes
  (`|ExecutionSequence`
    (:`then_0`
      (bind (_organe _axe) (`parent.tirer`))
      (set `local.cible` _organe)
      (switch `/Game/Manipulation/Enumérateurs/E_Axe` _axe
        (:`NewEnumerator0`
          _)
        (:`NewEnumerator1`
          _)
        (:`NewEnumerator2`
          _)
        (:`NewEnumerator4`
          _))
      ; On déplace l'organe (assemblage ou pièce) au plus proche du curseur de la souris
      (`|ExecutionSequence`
        (:`then_0`
          (set `local.positionFin` (`self.organeDeplacement` (`self.direction`))))
        (:`then_1`
          (`SceneComponent.K2_SetWorldLocation` (`local.cible`) _positionfin true false)
          (`self.K2_SetActorLocation` _positionfin false true))))
    (:`then_1`
      (return _organe _axe))))

(fn `UserConstructionScript`)