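; BP_Rotateur is a rotation gizmo with X, Y and Z pie handles (Camembert) for turning a robot part (organe) with the mouse.
; It extends a parent axes class, recording the part's rotation and projected cursor vector on anchoring.
; Dragging applies the signed Atan2 angle from that vector around the start rotation's local axis, to part and gizmo.
; LierStop forwards the used axis to the assembly's joint update.
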(fn `ancrageChanger`
  (params (organeAncre :type "SceneComponent Object Reference"))
  ; On retient les orientations de départ pour pouvoir les comparer ensuite
  (`parent.ancrageChanger` organeAncre)
  (switch `/Game/Manipulation/Enumérateurs/E_Axe` (`self.axeUtilise`)
    (:`NewEnumerator0`
      _)
    (:`NewEnumerator1`
      _)
    (:`NewEnumerator2`
      _)
    (:`NewEnumerator4`
      _))
  (set `self.departOrgane` (`SceneComponent.K2_GetComponentRotation` organeAncre))
  (bind _returnvalue (`GameplayStatics.GetActorOfClass` "/Game/Manipulation/Classes/Acteurs/Statiques/BP_Personnage.BP_Personnage_C"))
  (bind (_curseur _projectioncomposant) (`/Game/Manipulation/Classes/Acteurs/Statiques/BP_Personnage.curseurVecteur` _returnvalue (`self.DefaultSceneRoot`)))
  (set `self.departTirage` (- _curseur _projectioncomposant)))

(fn `axesInitialiser`
  (`parent.axesInitialiser`)
  (`|ExecutionSequence`
    (:`then_0`
      (`BlueprintMapLibrary.Map_Add` (`self.axes`) (`self.camembertX`) "NewEnumerator0"))
    (:`then_1`
      (`BlueprintMapLibrary.Map_Add` (`self.axes`) (`self.camembertY`) "NewEnumerator1"))
    (:`then_2`
      (`BlueprintMapLibrary.Map_Add` (`self.axes`) (`self.camembertZ`) "NewEnumerator2"))))

(fn `lierStop`
  (returns (assemblage :type "/Game/Manipulation/Classes/Acteurs/BP_Robot Object Reference") (pieceA :type "StaticMeshComponent Object Reference") (pieceB :type "StaticMeshComponent Object Reference"))
  (bind _axeutilise (`self.axeUtilise`))
  ; Prise en compte des paramètres : l'axe (x, y, z) et l'état de la contrainte (libre, limitée ou bloquée)
  (bind (_assemblage _piecea _pieceb) (`parent.lierStop`))
  (`/Engine/EditorBlueprintResources/StandardMacros.IsValid` _assemblage
    (:`Is Valid`
      (`|ExecutionSequence`
        (:`then_0`
          (switch `/Game/Manipulation/Enumérateurs/E_Axe` _axeutilise
            (:`NewEnumerator0`
              _)
            (:`NewEnumerator1`
              _)
            (:`NewEnumerator2`
              _)
            (:`NewEnumerator4`
              _))
          (`/Game/Manipulation/Classes/Acteurs/BP_Robot.liaisonChanger` :`self` _assemblage :`pieceA` _piecea :`pieceB` _pieceb :`transformation` "NewEnumerator1" :`axe` _axeutilise))
        (:`then_1`
          (return _assemblage _piecea _pieceb))))))

(fn `organeOrientation`
  (returns (angle :type "Float (double-precision)"))
  (bind _departtirage (`self.departTirage`))
  ; Angle entre le vecteur souris au départ de la rotation, et le vecteur souris actuel
  (bind _returnvalue (`GameplayStatics.GetActorOfClass` "/Game/Manipulation/Classes/Acteurs/Statiques/BP_Personnage.BP_Personnage_C"))
  (bind (_curseur _projectioncomposant) (`/Game/Manipulation/Classes/Acteurs/Statiques/BP_Personnage.curseurVecteur` _returnvalue (`self.DefaultSceneRoot`)))
  (bind _returnvalue_2 (- _curseur _projectioncomposant))
  (return (* (`KismetMathLibrary.DegAtan2` (`KismetMathLibrary.CrossProduct2D` _returnvalue_2 _departtirage) (`KismetMathLibrary.DotProduct2D` _departtirage _returnvalue_2)) -1.0)))

(fn `tirer`
  (returns (organe :type "SceneComponent Object Reference") (axe :type "/Game/Manipulation/Enumérateurs/E_Axe Enum"))
  (locals (rotationFin :type "Rotator Structure") (cible :type "SceneComponent Object Reference"))
  (bind _departorgane (`self.departOrgane`))
  (bind _rotationfin (`local.rotationFin`))
  (bind (_x _y _z) (`KismetMathLibrary.GetAxes` _departorgane))
  ; On tire sur un des trois axes
  (`|ExecutionSequence`
    (:`then_0`
      (bind (_organe _axe) (`parent.tirer`))
      (set `local.cible` _organe)
      (switch `/Game/Manipulation/Enumérateurs/E_Axe` _axe
        (:`NewEnumerator0`
          _)
        (:`NewEnumerator1`
          _)
        (:`NewEnumerator2`
          _)
        (:`NewEnumerator4`
          _))
      ; On oriente le robot au plus proche du curseur de la souris
      (`|ExecutionSequence`
        (:`then_0`
          (set `local.rotationFin` (`KismetMathLibrary.ComposeRotators` _departorgane (`KismetMathLibrary.RotatorFromAxisAndAngle` (select `/Game/Manipulation/Enumérateurs/E_Axe` (`self.axeUtilise`) :`NewEnumerator0` _x :`NewEnumerator1` _y :`NewEnumerator2` _z) (`self.organeOrientation`)))))
        (:`then_1`
          (`SceneComponent.K2_SetWorldRotation` (`local.cible`) _rotationfin true false)
          (`self.K2_SetActorRotation` _rotationfin true))))
    (:`then_1`
      (return _organe _axe))))

(fn `UserConstructionScript`)