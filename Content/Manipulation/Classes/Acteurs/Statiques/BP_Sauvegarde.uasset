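; BP_Sauvegarde handles persistence of robots and their imported 3D models under the project directory.
; Robot assemblies are stored in one JSON file keyed by robot name, with functions to list, read, write and delete entries.
; Importing checks the format, copies the model under a numbered name if needed, spawns a tagged BP_Robot before the camera and saves its placement and pieces.
; A name conflict can also rename the existing robot or model file.
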(fn `dossierModeles`
  (returns (cheminAbsolu :type String))
  (locals (cheminRelatif :type String :default "sauvegarde/modeles/"))
  ; Chemin vers le dossier des modèles 3D
  (return (`KismetStringLibrary.Concat_StrStr` (`KismetSystemLibrary.GetProjectDirectory`) (`local.cheminRelatif`))))

(fn `ecrire`
  (params (champ :type "/Game/Manipulation/Types/S_ChampRobot Structure"))
  (locals (contenu :type "JsonObjectWrapper Structure"))
  (bind (_champ_identifiant _champ_assemblage) (break `/Game/Manipulation/Types/S_ChampRobot` (`local.champ`)))
  (`|ExecutionSequence`
    (:`then_0`
      ; Sérialisation de l'identifiant du robot
      (bind _outjsonobject (`JsonBlueprintFunctionLibrary.FromFile` (make `FilePath` (`self.fichierSauvegarde`))))
      (bind _output_get (set `local.contenu` _outjsonobject))
      (`|SetJsonField` _output_get _champ_identifiant _champ_assemblage))
    (:`then_1`
      ; Écriture dans le fichier
      (`JsonBlueprintFunctionLibrary.ToFile` (`local.contenu`) (make `FilePath` (`self.fichierSauvegarde`))))))

(fn `ecrireSuppression`
  (params (assemblage :type "/Game/Manipulation/Classes/Acteurs/BP_Robot Object Reference"))
  (`/Engine/EditorBlueprintResources/StandardMacros.IsValid` assemblage
    (:`Is Valid`
      (`self.identifiantEcrireSuppression` (`/Game/Manipulation/Classes/Acteurs/BP_Robot.nomObtenir` assemblage)))))

(fn `fichierSauvegarde`
  (returns (cheminAbsolu :type String))
  (locals (cheminRelatif :type String :default "sauvegarde/robots.json"))
  ; Chemin vers le fichier de sauvegarde
  (return (`KismetStringLibrary.Concat_StrStr` (`KismetSystemLibrary.GetProjectDirectory`) (`local.cheminRelatif`))))

(fn `identifiantEcrireSuppression`
  (params (identifiant :type String))
  (locals (contenu :type "JsonObjectWrapper Structure"))
  (`|ExecutionSequence`
    (:`then_0`
      ; Sérialisation de tous les autres identifiants
      (bind _outjsonobject (`JsonBlueprintFunctionLibrary.FromFile` (make `FilePath` (`self.fichierSauvegarde`))))
      (bind _fieldnames (`JsonBlueprintFunctionLibrary.GetFieldNames` _outjsonobject))
      (for _array_element _fieldnames
        (if (`KismetStringLibrary.NotEqual_StrStr` _array_element (`local.identifiant`))
          (bind (_donnees_identifiant _donnees_assemblage) (break `/Game/Manipulation/Types/S_ChampRobot` (`self.identifiantLire` _array_element)))
          (`|SetJsonField` (`local.contenu`) _donnees_identifiant _donnees_assemblage))))
    (:`then_1`
      ; Écriture dans le fichier
      (`JsonBlueprintFunctionLibrary.ToFile` (`local.contenu`) (make `FilePath` (`self.fichierSauvegarde`))))))

(fn `identifiantLire`
  (params (identifiant :type String))
  (returns (donnees :type "/Game/Manipulation/Types/S_ChampRobot Structure"))
  ; On va chercher les informations sur le robot grâce à son identifiant
  (bind _outjsonobject (`JsonBlueprintFunctionLibrary.FromFile` (make `FilePath` (`self.fichierSauvegarde`))))
  (bind _outvalue (`|GetJsonField` _outjsonobject (`local.identifiant`)))
  (return (make `/Game/Manipulation/Types/S_ChampRobot` (`local.identifiant`) _outvalue)))

(fn `identifiantsObtenir`
  (returns (identifiants :type "Set of String"))
  (locals (identifiantsSauvegarde :type "Set of String"))
  ; Lecture depuis le fichier
  (bind _outjsonobject (`JsonBlueprintFunctionLibrary.FromFile` (make `FilePath` (`self.fichierSauvegarde`))))
  (bind _fieldnames (`JsonBlueprintFunctionLibrary.GetFieldNames` _outjsonobject))
  (for _array_element _fieldnames
    (`BlueprintSetLibrary.Set_Add` (`local.identifiantsSauvegarde`) _array_element))
  (return (`local.identifiantsSauvegarde`)))

(fn `lire`
  (params (assemblage :type "/Game/Manipulation/Classes/Acteurs/BP_Robot Object Reference"))
  (returns (donnees :type "/Game/Manipulation/Types/S_ChampRobot Structure"))
  ; On se sert du nom du robot comme son identifiant
  (`/Engine/EditorBlueprintResources/StandardMacros.IsValid` assemblage
    (:`Is Valid`
      (return (`self.identifiantLire` (`/Game/Manipulation/Classes/Acteurs/BP_Robot.nomObtenir` assemblage))))))

(fn `modeleCopier`
  (params (fichier :type String))
  (returns (copie :type String))
  (locals (existe :type Boolean :default true) (numero :type Integer :default 1) (formatConflit :type String) (formatCopie :type String) (nomConflit :type String) (nomCopie :type String))
  (bind (_pathpart _filenamepart _extensionpart) (`BlueprintPathsLibrary.Split` fichier))
  (bind _nomcopie (`local.nomCopie`))
  (bind _returnvalue (`BlueprintPathsLibrary.SetExtension` (`KismetStringLibrary.Concat_StrStr` (`self.dossierModeles`) (`local.nomCopie`)) (`local.formatCopie`)))
  (set `local.nomCopie` _filenamepart)
  (set `local.formatCopie` _extensionpart)
  (`|ExecutionSequence`
    (:`then_0`
      ; Tant que le nom existe déjà, on incrémente un numéro
      (bind _output_get (set `local.existe` (`self.modeleExiste` (`local.nomCopie`))))
      (while _output_get
        (bind _result (`/Engine/EditorBlueprintResources/StandardMacros.IncrementInt` (`local.numero`))
          (:`  `
            (bind (_existe _format) (`self.modeleExiste` (`/Game/Manipulation/Classes/Abstraites/BPFL_Caracteres.numeroAjouter` _result (`local.nomCopie`))))
            (set `local.existe` _existe)
            (set `local.formatConflit` _format)))))
    (:`then_1`
      ; S'il y a déjà un fichier au même nom, on lui ajoute un numéro pour rendre le nom unique
      (switch `int` (`local.numero`)
        (:`Default`
          (set `local.nomConflit` _nomcopie :!label _label)
          (set `local.nomCopie` (`/Game/Manipulation/Classes/Abstraites/BPFL_Caracteres.numeroAjouter` (`local.numero`) _nomcopie)))
        (:`0`
          (`/Game/Manipulation/Classes/Abstraites/BPFL_Caracteres.erreurAfficher` "nombre négatif d'occurences"))
        (:`2`
          (`|ExecutionSequence`
            (:`then_0`
              (goto _label))
            (:`then_1`
              (bind _outactors (`GameplayStatics.GetAllActorsOfClassWithTag` "/Game/Manipulation/Classes/Acteurs/BP_Robot.BP_Robot_C" (`KismetStringLibrary.Conv_StringToName` (`local.nomConflit`))))
              (if (`KismetArrayLibrary.Array_IsEmpty` _outactors)
                (`self.modeleRenommer` (`BlueprintPathsLibrary.SetExtension` (`local.nomCopie`) (`local.formatCopie`)) (`BlueprintPathsLibrary.SetExtension` (`local.nomConflit`) (`local.formatConflit`)))
                (else
                  (`/Game/Manipulation/Classes/Acteurs/BP_Robot.renommer` (`|GetArrayItem` _outactors) (`local.nomCopie`)))))))))
    (:`then_2`
      ; On copie l'ancien fichier dans le dossier de sauvegarde des modèles
      (`BlueprintFileUtilsBPLibrary.CopyFile` _returnvalue (`local.fichier`) false true)
      (return _returnvalue))))

(fn `modeleExiste`
  (params (nom :type String))
  (returns (existe :type Boolean) (format :type String))
  (bind _valuepin (`|SetForEach` (`self.formatsModeles`))
    (:`then`
      ; On teste l'existence du nom de fichier avec tous les formats possibles
      (bind _returnvalue (`BlueprintFileUtilsBPLibrary.FileExists` (`BlueprintPathsLibrary.SetExtension` (`KismetStringLibrary.Concat_StrStr` (`self.dossierModeles`) (`local.nom`)) _valuepin)))
      (if _returnvalue
        (return _returnvalue _valuepin)))
    (:`CompletedPin`
      (return false ""))))

(fn `modeleImporter`
  (params (cheminFichier :type String))
  (locals (nouvelAssemblage :type "/Game/Manipulation/Classes/Acteurs/BP_Robot Object Reference") (copieChemin :type String) (copieExtension :type String) (copieNom :type String) (nouvellesPieces :type "Map of String to /Game/Manipulation/Types/S_Piece Structure") (transformationDepart :type "Transform Structure" :default "0.000000,-1000.000000,0.000000|0.000000,0.000000,0.000000|1.000000,1.000000,1.000000"))
  (bind _copiechemin (`local.copieChemin`))
  (if (`/Game/Manipulation/Classes/Abstraites/BPFL_Caracteres.formatVerifier` cheminFichier (`self.formatsModeles`))
    (`|ExecutionSequence`
      (:`then_0`
        ; On fait une copie du modèle, au cas où l'utilisateur supprimerait son exemplaire
        (bind _copie (`self.modeleCopier` (`local.cheminFichier`)))
        (set `local.copieChemin` _copie))
      (:`then_1`
        ; On donne un nom au robot
        (set `local.copieNom` (`BlueprintPathsLibrary.GetBaseFilename` _copiechemin))
        (set `local.copieExtension` (`BlueprintPathsLibrary.GetExtension` _copiechemin)))
      (:`then_2`
        ; Le robot apparaît devant la caméra
        (bind _returnvalue (`GameplayStatics.GetActorOfClass` "/Game/Manipulation/Classes/Acteurs/Statiques/BP_Personnage.BP_Personnage_C"))
        (bind _returnvalue_2 (`GameplayStatics.GetActorOfClass` "/Game/Manipulation/Classes/Acteurs/Statiques/BP_Logiciel.BP_Logiciel_C"))
        (bind (_returnvalue_location _returnvalue_rotation) (`KismetMathLibrary.BreakTransform` (`SceneComponent.K2_GetComponentToWorld` (`/Game/Manipulation/Classes/Acteurs/Statiques/BP_Personnage.camera` _returnvalue))))
        (bind _output_get (set `local.transformationDepart` (`KismetMathLibrary.MakeTransform` (+ (`KismetMathLibrary.GreaterGreater_VectorRotator` (`KismetMathLibrary.MakeVector` (`/Game/Manipulation/Classes/Acteurs/Statiques/BP_Logiciel.tailleUtilisateur` _returnvalue_2)) _returnvalue_rotation) _returnvalue_location) _returnvalue_rotation)))
        (bind _returnvalue_3 (`|SpawnActorFromClass` "/Game/Manipulation/Classes/Acteurs/BP_Robot.BP_Robot_C" _output_get "Undefined" "MultiplyWithRoot" null (`|MakeArray` (`KismetStringLibrary.Conv_StringToName` (`local.copieNom`))) null))
        (set `local.nouvelAssemblage` _returnvalue_3))
      (:`then_3`
        ; On sauvegarde le chemin vers le modèle copié ainsi que les pièces générées
        (bind (_arrayindex _arrayelement) (`/Engine/EditorBlueprintResources/StandardMacros.ReverseForEachLoop` (`self.K2_GetComponentsByClass` (`local.nouvelAssemblage`) "/Script/Engine.StaticMeshComponent"))
          (:`LoopBody`
            (`BlueprintMapLibrary.Map_Add` (`local.nouvellesPieces`) (`/Game/Manipulation/Classes/Abstraites/BPFL_Piece.nomObtenir` _arrayelement) (make `/Game/Manipulation/Types/S_Piece` (`/Game/Manipulation/Classes/Abstraites/BPFL_Transformation.transformationVersPlacement` (`SceneComponent.GetRelativeTransform` _arrayelement)))))
          (:`Completed`
            (`self.ecrire` (make `/Game/Manipulation/Types/S_ChampRobot` (`local.copieNom`) (make `/Game/Manipulation/Types/S_Assemblage` (`local.copieExtension`) (`/Game/Manipulation/Classes/Abstraites/BPFL_Transformation.transformationVersPlacement` (`local.transformationDepart`)) (`local.nouvellesPieces`)))))))
      (:`then_4`
        ; Affichage console
        (`KismetSystemLibrary.PrintText` (`|FormatText` "{modeleCopie} importé" (`local.copieNom`)) true true (`/Game/Manipulation/Classes/Abstraites/BPFL_Couleur.jaune`) 10.0)))
    (else
      ; Erreur : mauvais format
      (`/Game/Manipulation/Classes/Abstraites/BPFL_Caracteres.erreurAfficher` (`|FormatText` "les formats de modèles 3D pris en charge sont {formats}" (`/Game/Manipulation/Classes/Abstraites/BPFL_Caracteres.ensembleJoindre` (`self.formatsModeles`) ", "))))))

(fn `modeleRenommer`
  (params (nomNouveau :type String) (nomAncien :type String))
  (bind _cheminabsolu (`self.dossierModeles`))
  (bind _returnvalue (`KismetStringLibrary.Concat_StrStr` _cheminabsolu nomAncien))
  (`BlueprintFileUtilsBPLibrary.CopyFile` (`KismetStringLibrary.Concat_StrStr` _cheminabsolu nomNouveau) _returnvalue false true)
  (`BlueprintFileUtilsBPLibrary.DeleteFile` _returnvalue true true))

(fn `UserConstructionScript`)