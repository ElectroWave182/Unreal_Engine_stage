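; BP_Personnage is the player pawn for both desktop mouse and VR headset, handling movement, aiming, snap turns and selection.
; Cursor helpers switch between mouse and motion-controller laser, which updates hover in BP_Logiciel each Tick.
; Selection presses the controller's widget pointer, re-anchors BP_Logiciel's transformer and clicks the hovered part.
; In VR, yaw on the actor, headset rotation on GyroscopeCasque and pitch on Camera stack to allow joystick turning.
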(event `self.ReceiveBeginPlay`
  (bind _returnvalue (`GameplayStatics.GetPlayerController` 0))
  (if (`HeadMountedDisplayFunctionLibrary.IsHeadMountedDisplayEnabled`)
    (`|ExecutionSequence`
      (:`then_0`
        ; Le traçage commence sur le personnage, en réalité virtuelle
        (`HeadMountedDisplayFunctionLibrary.SetTrackingOrigin` "Local")
        ; Résolution (en pourcentage)
        (`KismetSystemLibrary.ExecuteConsoleCommand` "xr.SecondaryScreenPercentage.HMDRenderTarget 100" null)
        (`XRLoadingScreenFunctionLibrary.HideLoadingScreen`))
      (:`then_1`
        ; En réalité virtuelle, la souris est désactivée
        (set `PlayerController.bEnableClickEvents` false _returnvalue)
        (set `PlayerController.bEnableMouseOverEvents` false _returnvalue)
        (set `PlayerController.bShowMouseCursor` false _returnvalue))
      (:`then_2`
        ; Affichage console
        (`KismetSystemLibrary.PrintText` "Casque de réalité virtuelle reconnu" true true (`/Game/Manipulation/Classes/Abstraites/BPFL_Couleur.blanc`) 10.0)))))

(event `self.ReceiveTick`
  (params (DeltaSeconds :type "Float (single-precision)"))
  ; Boucle
  (if (`HeadMountedDisplayFunctionLibrary.IsHeadMountedDisplayEnabled`)
    (`self.gyroscopePointer` (`self.mainPrincipale`))))

(event `EnhancedInput|/Game/Manipulation/Contrôles/Principal/Actions/IA_Mouvement`
  (params (ActionValue :type "Vector Structure") (ElapsedSeconds :type "Float (double-precision)") (TriggeredSeconds :type "Float (double-precision)") (InputAction :type "InputAction Object Reference" :default "/Game/Manipulation/Contrôles/Principal/Actions/IA_Mouvement.IA_Mouvement"))
  ; Commandes
  (:`Triggered`
    (`self.bouger` ActionValue)))

(event `EnhancedInput|/Game/Manipulation/Contrôles/Principal/Actions/IA_CameraConditionnelle`
  (params (ActionValue :type "Vector2D Structure") (ElapsedSeconds :type "Float (double-precision)") (TriggeredSeconds :type "Float (double-precision)") (InputAction :type "InputAction Object Reference" :default "/Game/Manipulation/Contrôles/Principal/Actions/IA_CameraConditionnelle.IA_CameraConditionnelle"))
  ; Commandes
  (:`Triggered`
    (if (`|GetInputActionValue`)
      (`self.viser` ActionValue_X ActionValue_Y))))

(event `EnhancedInput|/Game/Manipulation/Contrôles/Principal/Actions/IA_Camera`
  (params (ActionValue :type "Vector2D Structure") (ElapsedSeconds :type "Float (double-precision)") (TriggeredSeconds :type "Float (double-precision)") (InputAction :type "InputAction Object Reference" :default "/Game/Manipulation/Contrôles/Principal/Actions/IA_Camera.IA_Camera"))
  ; Commandes
  (:`Triggered`
    (`self.viser` ActionValue_X ActionValue_Y)))

(event `EnhancedInput|/Game/Manipulation/Contrôles/Principal/Actions/IA_CameraCrantee`
  (params (ActionValue :type "Float (double-precision)") (ElapsedSeconds :type "Float (double-precision)") (TriggeredSeconds :type "Float (double-precision)") (InputAction :type "InputAction Object Reference" :default "/Game/Manipulation/Contrôles/Principal/Actions/IA_CameraCrantee.IA_CameraCrantee"))
  ; Commandes
  (:`Started`
    (`self.viserInstantanement` (> ActionValue 0.0))))

(event `EnhancedInput|/Game/Manipulation/Contrôles/Principal/Actions/IA_Recalibrage`
  (params (ActionValue :type "Float (double-precision)") (ElapsedSeconds :type "Float (double-precision)") (TriggeredSeconds :type "Float (double-precision)") (InputAction :type "InputAction Object Reference" :default "/Game/Manipulation/Contrôles/Principal/Actions/IA_Recalibrage.IA_Recalibrage"))
  ; Commandes
  (:`Started`
    (bind _enumvalue (foreach `/Game/Manipulation/Enumérateurs/E_Main` false)
      (:`LoopBody`
        (`self.gyroscopeRecalibrer` _enumvalue)))))

(event `EnhancedInput|/Game/Manipulation/Contrôles/Principal/Actions/IA_Selection`
  (params (ActionValue :type "Float (double-precision)") (ElapsedSeconds :type "Float (double-precision)") (TriggeredSeconds :type "Float (double-precision)") (InputAction :type "InputAction Object Reference" :default "/Game/Manipulation/Contrôles/Principal/Actions/IA_Selection.IA_Selection"))
  (bind _touche (`self.toucheObtenir` "/Game/Manipulation/Contrôles/Principal/Actions/IA_Selection.IA_Selection"))
  (bind _manette (`self.manetteObtenir` (`self.mainPrincipale`)))
  ; Commandes
  (:`Started`
    (`WidgetInteractionComponent.PressPointerKey` _manette _touche)
    (`|ExecutionSequence`
      (:`then_0`
        (bind _returnvalue (`GameplayStatics.GetActorOfClass` "/Game/Manipulation/Classes/Acteurs/Statiques/BP_Logiciel.BP_Logiciel_C"))
        (bind _organenettoye (`/Game/Manipulation/Classes/Acteurs/Statiques/BP_Logiciel.selectionNettoyer` _returnvalue))
        (`/Game/Manipulation/Classes/Acteurs/Statiques/Axes/BP_Transformateur.ancrageChanger` (`/Game/Manipulation/Classes/Acteurs/Statiques/BP_Logiciel.transformateur` _returnvalue) _organenettoye)
        (bind _organesurvole (`/Game/Manipulation/Classes/Acteurs/Statiques/BP_Logiciel.organeSurvole` _returnvalue))
        (`/Engine/EditorBlueprintResources/StandardMacros.IsValid` _organesurvole
          (:`Is Valid`
            (`/Game/Manipulation/Classes/Acteurs/BP_Robot.clic` (`/Game/Manipulation/Classes/Acteurs/Statiques/BP_Logiciel.assemblageSurvole` _returnvalue) _organesurvole))))
      (:`then_1`
        (set `self.coordonneesSelection` (`self.curseurVecteur` null)))))
  (:`Completed`
    (`WidgetInteractionComponent.ReleasePointerKey` _manette _touche)
    (bind _returnvalue_2 (`GameplayStatics.GetActorOfClass` "/Game/Manipulation/Classes/Acteurs/Statiques/BP_Logiciel.BP_Logiciel_C"))
    (`/Game/Manipulation/Classes/Acteurs/Statiques/Axes/BP_Transformateur.lacher` (`/Game/Manipulation/Classes/Acteurs/Statiques/BP_Logiciel.transformateur` _returnvalue_2))))

(fn `bouger`
  (params (direction :type "Vector Structure" :default (1.0 0.0 0.0)))
  (bind _camera (`self.camera`))
  (bind (_returnvalue_x _returnvalue_y) (`KismetMathLibrary.BreakVector` (`SceneComponent.GetForwardVector` _camera)))
  ; Droite / Gauche
  (`self.AddMovementInput` (`SceneComponent.GetRightVector` _camera) direction_X)
  ; Haut / Bas
  (`self.AddMovementInput` (`KismetMathLibrary.GetUpVector` (struct)) direction_Y)
  ; Devant / Derrière
  (`self.AddMovementInput` (`KismetMathLibrary.Normal` (`KismetMathLibrary.MakeVector` _returnvalue_x _returnvalue_y)) direction_Z))

(fn `curseurCollision`
  (params (canal :type "ETraceTypeQuery Enum" :default "TraceTypeQuery1"))
  (returns (impact :type "Vector Structure") (touche :type "PrimitiveComponent Object Reference"))
  (bind _hitresult (`PlayerController.GetHitResultUnderCursorByChannel` (`GameplayStatics.GetPlayerController` 0) (`local.canal`) true))
  (if (`HeadMountedDisplayFunctionLibrary.IsHeadMountedDisplayEnabled`)
    ; Mode manette
    (bind _outhit (`KismetSystemLibrary.LineTraceSingle` :`Start` (`SceneComponent.K2_GetComponentLocation` (`self.camera`)) :`End` (`self.curseurPlacement`) :`TraceChannel` (`local.canal`) :`bTraceComplex` true :`DrawTime` 10.0))
    (return (`.ImpactPoint` (`GameplayStatics.BreakHitResult` _outhit)) (`.HitComponent` (`GameplayStatics.BreakHitResult` _outhit)))
    (else
      ; Mode souris
      (return (`.ImpactPoint` (`GameplayStatics.BreakHitResult` _hitresult)) (`.HitComponent` (`GameplayStatics.BreakHitResult` _hitresult))))))

(fn `curseurPlacement`
  (returns (position :type "Vector Structure") (direction :type "Vector Structure"))
  (bind _mainprincipale (`self.mainPrincipale`))
  (bind _gyroscope (`self.gyroscopeObtenir` _mainprincipale))
  (bind (_worldlocation _worlddirection) (`PlayerController.DeprojectMousePositionToWorld` (`GameplayStatics.GetPlayerController` 0)))
  (bind _returnvalue (+ (`SceneComponent.K2_GetComponentLocation` _gyroscope) (* (`KismetMathLibrary.Conv_RotatorToVector` (`SceneComponent.K2_GetComponentRotation` _gyroscope)) (`WidgetInteractionComponent.InteractionDistance` (`self.manetteObtenir` _mainprincipale)))))
  (if (`HeadMountedDisplayFunctionLibrary.IsHeadMountedDisplayEnabled`)
    ; Mode manette
    (return _returnvalue (- _returnvalue (`SceneComponent.K2_GetComponentLocation` (`self.camera`))))
    (else
      ; Mode souris
      (return _worldlocation _worlddirection))))

(fn `curseurVecteur`
  (params (composant :type "SceneComponent Object Reference"))
  (returns (curseur :type "Vector2D Structure") (projectionComposant :type "Vector2D Structure"))
  (locals (projection :type "Vector2D Structure"))
  (bind _returnvalue (`GameplayStatics.GetPlayerController` 0))
  (bind _composant (`local.composant`))
  (bind (_locationx _locationy) (`PlayerController.GetMousePosition` _returnvalue))
  ; Vecteur de l'origine projetée sur l'écran vers le curseur
  (`|ExecutionSequence`
    (:`then_0`
      (`/Engine/EditorBlueprintResources/StandardMacros.IsValid` _composant
        (:`Is Valid`
          (set `local.projection` (`GameplayStatics.ProjectWorldToScreen` (`GameplayStatics.GetPlayerController` 0) (`SceneComponent.K2_GetComponentLocation` _composant))))))
    (:`then_1`
      (return (select `bool` (`HeadMountedDisplayFunctionLibrary.IsHeadMountedDisplayEnabled`) :`false` (`KismetMathLibrary.MakeVector2D` _locationx _locationy) :`true` (`GameplayStatics.ProjectWorldToScreen` _returnvalue (`self.curseurPlacement`))) (`local.projection`)))))

(fn `gyroscopeObtenir`
  (params (main :type "/Game/Manipulation/Enumérateurs/E_Main Enum" :default "NewEnumerator0"))
  (returns (gyroscope :type "MotionControllerComponent Object Reference"))
  (return (select `/Game/Manipulation/Enumérateurs/E_Main` main :`NewEnumerator0` (`self.MotionControllerRightAim`) :`NewEnumerator1` (`self.MotionControllerLeftAim`))))

(fn `gyroscopePointer`
  (params (main :type "/Game/Manipulation/Enumérateurs/E_Main Enum" :default "NewEnumerator0"))
  (bind _main (`local.main`))
  (`|ExecutionSequence`
    (:`then_0`
      ; En réalité virtuelle, on fait bouger un pointeur laser pour indiquer le survol
      (`SceneComponent.SetHiddenInGame` (`self.indicateurObtenir` _main) (not (`MotionControllerComponent.IsTracked` (`self.gyroscopeObtenir` _main))) false)
      (bind _returnvalue (`GameplayStatics.GetActorOfClass` "/Game/Manipulation/Classes/Acteurs/Statiques/BP_Logiciel.BP_Logiciel_C"))
      (`/Game/Manipulation/Classes/Acteurs/Statiques/BP_Logiciel.survolRemplacer` _returnvalue (`.touche` (`self.curseurCollision` "TraceTypeQuery1"))))
    (:`then_1`
      ;[1 0.5 0 0.5] Attention : on applique les rotations du casque sur l'acteur, pour pouvoir tourner la caméra de façon neutre avec le joystick (ne pas remplacer par "Lock to HMD")
      (bind _hmddata (`HeadMountedDisplayFunctionLibrary.GetHMDData` null))
      (`SceneComponent.K2_SetRelativeRotation` (`self.gyroscopeCasque`) (`KismetMathLibrary.Quat_Rotator` (`.Rotation` (break `XRHMDData` _hmddata))) false true))))

(fn `gyroscopeRecalibrer`
  (params (main :type "/Game/Manipulation/Enumérateurs/E_Main Enum" :default "NewEnumerator0"))
  (bind _returnvalue (`SceneComponent.K2_GetComponentRotation` (`self.gyroscopeObtenir` main)))
  ; On calibre le gyroscope pour le pointage
  (switch `/Game/Manipulation/Enumérateurs/E_Main` main
    (:`NewEnumerator0`
      (set `self.gyroscopeBaseDroite` _returnvalue))
    (:`NewEnumerator1`
      (set `self.gyroscopeBaseGauche` _returnvalue))))

(fn `indicateurObtenir`
  (params (main :type "/Game/Manipulation/Enumérateurs/E_Main Enum" :default "NewEnumerator0"))
  (returns (indicateur :type "StaticMeshComponent Object Reference"))
  (return (select `/Game/Manipulation/Enumérateurs/E_Main` main :`NewEnumerator0` (`self.indicateurDroit`) :`NewEnumerator1` (`self.indicateurGauche`))))

(fn `manetteObtenir`
  (params (main :type "/Game/Manipulation/Enumérateurs/E_Main Enum" :default "NewEnumerator0"))
  (returns (manette :type "WidgetInteractionComponent Object Reference"))
  (return (select `/Game/Manipulation/Enumérateurs/E_Main` main :`NewEnumerator0` (`self.WidgetInteractionRight`) :`NewEnumerator1` (`self.WidgetInteractionLeft`))))

(fn `toucheObtenir`
  (params (action :type "InputAction Object Reference"))
  (returns (touche :type "Key Structure"))
  ; Première touche associée à l'action
  (return (`|GetArrayItem` (`EnhancedInputSubsystemInterface.QueryKeysMappedToAction` (pcsubsystem `EnhancedInputLocalPlayerSubsystem` (`GameplayStatics.GetPlayerController` 0)) action))))

(fn `UserConstructionScript`)

(fn `viseeLimiter`
  (bind _returnvalue (`GameplayStatics.GetPlayerCameraManager` 0))
  (bind _camera (`self.camera`))
  (bind (_relativerotation_roll _relativerotation_pitch) (`KismetMathLibrary.BreakRotator` (`SceneComponent.RelativeRotation` _camera)))
  ; On restreint le tangage de la caméra
  (`SceneComponent.K2_SetRelativeRotation` _camera (`KismetMathLibrary.MakeRotator` 0.0 (`KismetMathLibrary.FClamp` _relativerotation_pitch (`PlayerCameraManager.ViewPitchMin` _returnvalue) (`PlayerCameraManager.ViewPitchMax` _returnvalue))) false true))

(fn `viser`
  (params (lacet :type "Float (single-precision)") (tangage :type "Float (double-precision)"))
  (bind (_returnvalue_roll _returnvalue_pitch) (`KismetMathLibrary.BreakRotator` (`self.K2_GetActorRotation`)))
  (bind _returnvalue (`GameplayStatics.GetPlayerCameraManager` 0))
  (bind _returnvalue_2 (< (`local.tangage`) 0.0))
  ; Droite / Gauche
  (`self.AddControllerYawInput` lacet)
  (if (`HeadMountedDisplayFunctionLibrary.IsHeadMountedDisplayEnabled`)
    ; Le "sandwich" : l'acteur qui gère le lacet est parent du composant qui gère le gyroscope du caque, qui est lui-même parent de la caméra, à laquelle on applique le tangage
    (`SceneComponent.K2_AddRelativeRotation` (`self.camera`) (`KismetMathLibrary.MakeRotator` 0.0 (`local.tangage`)) false true)
    (`self.viseeLimiter`)
    (elif (or (and (< (`PlayerCameraManager.ViewPitchMin` _returnvalue) _returnvalue_pitch) (not _returnvalue_2)) (and _returnvalue_2 (< _returnvalue_pitch (`PlayerCameraManager.ViewPitchMax` _returnvalue))))
      ; Haut / Bas
      (`self.AddControllerPitchInput` (`local.tangage`)))))

(fn `viserInstantanement`
  (params (coteDroit :type Boolean))
  (locals (angleCameraCrantee :type "Float (double-precision)" :default 30.0))
  (bind (_returnvalue_location _returnvalue_rotation) (`KismetMathLibrary.BreakTransform` (`self.GetTransform`)))
  (bind _camera (`self.camera`))
  (bind _anglecameracrantee (`local.angleCameraCrantee`))
  (bind _returnvalue (select `bool` (`local.coteDroit`) :`false` (* _anglecameracrantee -1.0) :`true` _anglecameracrantee))
  (bind _returnvalue_location_2 (`KismetMathLibrary.BreakTransform` (`KismetMathLibrary.ComposeTransforms` (`SceneComponent.GetRelativeTransform` _camera) (`KismetMathLibrary.MakeTransform` _returnvalue_location (`KismetMathLibrary.ComposeRotators` _returnvalue_rotation (`KismetMathLibrary.MakeRotator` 0.0 0.0 _returnvalue))))))
  ; On pivote instantanément le personnage de 30°, et on le décale pour donner l'impression qu'on tourne autour de la caméra (même fonction que SnapTurn d'Unreal Engine)
  (`self.K2_AddActorWorldOffset` (- (`SceneComponent.K2_GetComponentLocation` _camera) _returnvalue_location_2) false true)
  (`self.AddControllerYawInput` _returnvalue))