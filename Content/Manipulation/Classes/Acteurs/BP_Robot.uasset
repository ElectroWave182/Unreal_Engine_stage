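; Robot actor acting as a digital twin: a selectable, editable assembly of physics-simulated parts linked by constraints.
; Loads the glTF model named by its first tag at runtime, building one mesh component per node, placed from BP_Sauvegarde data when available.
; Joint edits feed BP_GrapheLiaisons and the JSON save, while real-robot movements from BP_Requetage drive joint motors.
; Hover and selection highlight parts with linked neighbours and drive BP_Logiciel's transformer.
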(event `self.ReceiveBeginPlay`
  (set `self.Tags` (`self.initialisationTags`))
  (`self.modeleCharger`)
  ; Événements de sélection, de suvrol et de collision
  (for _array_element (`self.K2_GetComponentsByClass` "/Script/Engine.StaticMeshComponent")
    (add `PrimitiveComponent.OnEndCursorOver` _array_element (delegate `survolFin`))
    (add `PrimitiveComponent.OnBeginCursorOver` _array_element (delegate `survolDebut`))))

(event `survolDebut`
  (params (TouchedComponent :type "PrimitiveComponent Object Reference"))
  ; Un organe (assemblage ou pièce) est surligné lorqu'on passe le curseur dessus
  (bind _returnvalue (`GameplayStatics.GetActorOfClass` "/Game/Manipulation/Classes/Acteurs/Statiques/BP_Logiciel.BP_Logiciel_C"))
  (bind (_estlie _estsurvole _esttire) (`/Game/Manipulation/Classes/Acteurs/Statiques/Axes/BP_Transformateur.utilisation` (`/Game/Manipulation/Classes/Acteurs/Statiques/BP_Logiciel.transformateur` _returnvalue)))
  (if (not (or _estsurvole _esttire))
    (`self.survolDefinir` true TouchedComponent)))

(event `survolFin`
  (params (TouchedComponent :type "PrimitiveComponent Object Reference"))
  ; Un organe (assemblage ou pièce) est surligné lorqu'on passe le curseur dessus
  (`self.survolDefinir` false TouchedComponent))

(fn `clic`
  (params (organeClique :type "SceneComponent Object Reference"))
  ; Un clic sur un organe (assemblage ou pièce) désélectionne tout, puis sélectionne cet organe
  (bind _returnvalue (`GameplayStatics.GetActorOfClass` "/Game/Manipulation/Classes/Acteurs/Statiques/BP_Logiciel.BP_Logiciel_C"))
  (bind (_estlie _estsurvole _esttire) (`/Game/Manipulation/Classes/Acteurs/Statiques/Axes/BP_Transformateur.utilisation` (`/Game/Manipulation/Classes/Acteurs/Statiques/BP_Logiciel.transformateur` _returnvalue)))
  (if (not (or _estlie _estsurvole _esttire))
    (`self.selectionDefinir` true organeClique)))

(fn `estSelectionneOuLie`
  (params (organe :type "SceneComponent Object Reference"))
  (returns (est :type Boolean))
  (locals (logiciel :type "/Game/Manipulation/Classes/Acteurs/Statiques/BP_Logiciel Object Reference"))
  (bind _returnvalue (== (`/Game/Manipulation/Classes/Acteurs/Statiques/BP_Logiciel.organeSelectionne` (`local.logiciel`)) (`local.organe`)))
  (bind _returnvalue_2 (`GameplayStatics.GetActorOfClass` "/Game/Manipulation/Classes/Acteurs/Statiques/BP_Logiciel.BP_Logiciel_C"))
  (set `local.logiciel` _returnvalue_2)
  (bind _asstatic_mesh_component (cast `StaticMeshComponent` (`local.organe`))
    (:`then`
      (bind _asstatic_mesh_component_2 (cast `StaticMeshComponent` (`/Game/Manipulation/Classes/Acteurs/Statiques/BP_Logiciel.organeSelectionne` (`local.logiciel`)))
        (:`then`
          ; S'il s'agit d'une pièce de robot, il faut aussi vérifier ses pièces liées
          (return (or (`BlueprintMapLibrary.Map_Contains` (break `/Game/Manipulation/Types/S_PiecesLiees` (`BlueprintMapLibrary.Map_Find` (`/Game/Manipulation/Classes/Acteurs/BP_GrapheLiaisons.adjacences` (`self.liaisons`)) _asstatic_mesh_component_2)) _asstatic_mesh_component) _returnvalue)))
        (:`CastFailed`
          _)))
    (:`CastFailed`
      _))
  ; S'il s'agit d'un assemblage entier, il ne peut pas avoir de liaisons
  (return _returnvalue))

(fn `liaisonChanger`
  (params (nouvelleLiaison :type "/Game/Manipulation/Types/S_Liaison Structure") (pieceA :type "StaticMeshComponent Object Reference") (pieceB :type "StaticMeshComponent Object Reference") (transformation :type "/Game/Manipulation/Enumérateurs/E_Transformation Enum" :default "NewEnumerator0") (axe :type "/Game/Manipulation/Enumérateurs/E_Axe Enum" :default "NewEnumerator0"))
  (locals (liaison :type "Map of /Game/Manipulation/Enumérateurs/E_Transformation Enum to /Game/Manipulation/Types/S_ContraintesAxes Structure") (etatPhysiqueNouveau :type "/Game/Manipulation/Types/S_Physique Structure") (nomA :type String) (nomB :type String) (pieces :type "Map of String to /Game/Manipulation/Types/S_Piece Structure") (pieceLiaisons :type "Map of String to /Game/Manipulation/Types/S_Liaison Structure") (pieceTransformation :type "Transform Structure"))
  (bind _noma (`local.nomA`))
  (bind _nomb (`local.nomB`))
  (bind (_nouvelleliaison_placement _nouvelleliaison_contraintes) (break `/Game/Manipulation/Types/S_Liaison` (`local.nouvelleLiaison`)))
  (bind _transformation (`local.transformation`))
  (bind _axe (`local.axe`))
  (bind _liaison (`local.liaison`))
  (bind _liaisons (`self.liaisons`))
  (bind (_nouvelleliaison_placement_2 _nouvelleliaison_contraintes_2) (break `/Game/Manipulation/Types/S_Liaison` (`local.nouvelleLiaison`)))
  (bind _piecea (`local.pieceA`))
  (bind _transformation_2 (`local.transformation`))
  (bind _pieceb (`local.pieceB`))
  (bind _nouvelleliaison_placement_3 (break `/Game/Manipulation/Types/S_Liaison` (`local.nouvelleLiaison`)))
  (bind _axe_2 (`local.axe`))
  (bind _pieceb_2 (`local.pieceB`))
  (bind _value (`BlueprintMapLibrary.Map_Find` _liaison _transformation_2))
  (bind _value_2 (`BlueprintMapLibrary.Map_Find` (`local.pieces`) (`local.nomA`)))
  (bind (_value_3 _returnvalue) (`BlueprintMapLibrary.Map_Find` (`.liaisons_7_45728FC442F8D33DC8BA7A8E1B036B66` (break `/Game/Manipulation/Types/S_Piece` _value_2)) (`local.nomB`)))
  (`|ExecutionSequence`
    (:`then_0`
      ; Récupération des informations depuis la sauvegarde
      (bind _returnvalue_2 (`GameplayStatics.GetActorOfClass` "/Game/Manipulation/Classes/Acteurs/Statiques/BP_Sauvegarde.BP_Sauvegarde_C"))
      (set `local.pieces` (`.pieces_15_AA0EACB64195D6F1CD7D1B8D3DEB6A4A` (break `/Game/Manipulation/Types/S_Assemblage` (`.assemblage_5_ABD141CF4D373683774A5881ABCE92B3` (break `/Game/Manipulation/Types/S_ChampRobot` (`/Game/Manipulation/Classes/Acteurs/Statiques/BP_Sauvegarde.lire` _returnvalue_2 self)))))))
    (:`then_1`
      ; On vient chercher la liaison existante
      (set `local.nomA` (`/Game/Manipulation/Classes/Abstraites/BPFL_Piece.nomObtenir` (`local.pieceA`)))
      (`/Engine/EditorBlueprintResources/StandardMacros.IsValid` _pieceb_2
        (:`Is Valid`
          (set `local.nomB` (`/Game/Manipulation/Classes/Abstraites/BPFL_Piece.nomObtenir` _pieceb_2))
          (if (== (`ActorComponent.GetOwner` (`local.pieceA`)) (`ActorComponent.GetOwner` (`local.pieceB`)))
            (set `local.pieceTransformation` (`/Game/Manipulation/Classes/Abstraites/BPFL_Transformation.placementVersTransformation` (break `/Game/Manipulation/Types/S_Piece` _value_2)) :!label _label)
            (set `local.pieceLiaisons` (`.liaisons_7_45728FC442F8D33DC8BA7A8E1B036B66` (break `/Game/Manipulation/Types/S_Piece` _value_2)))
            ; S'il n'y en a pas, on part d'une liaison libre
            (if _returnvalue
              (set `local.liaison` (`.contraintes_7_147DBC5940D797B1F538718E58A09DF9` (break `/Game/Manipulation/Types/S_Liaison` _value_3)))
              (else
                (set `local.liaison` (`/Game/Manipulation/Classes/Abstraites/BPFL_Contrainte.liaisonParfaite` "NewEnumerator12"))))
            (else
              ; Erreur : assemblages différents
              (`/Game/Manipulation/Classes/Abstraites/BPFL_Caracteres.erreurAfficher` (`|FormatText` "impossible de changer la liaison, car la pièce {pieceB} n'est pas dans le même assemblage que {pieceA}" (`local.nomB`) (`local.nomA`))))))
        (:`Is Not Valid`
          (set `local.nomB` (`local.nomA`))
          (goto _label))))
    (:`then_2`
      (if (`BlueprintMapLibrary.Map_IsEmpty` _nouvelleliaison_contraintes_2)
        ; Si l'on a pas spécifié de nouvelles contraintes, une liaison libre devient bloquante, et inversement
        (switch `/Game/Manipulation/Enumérateurs/E_Axe` _axe_2
          (:`NewEnumerator0`
            (bind _output_get (set `local.etatPhysiqueNouveau` (`/Game/Manipulation/Classes/Abstraites/BPFL_Contrainte.physiqueInverser` (`/Game/Manipulation/Classes/Abstraites/BPFL_Contrainte.etatPhysiqueObtenir` _liaison _transformation_2 _axe_2)) :!label _label_2))
            (`/Game/Manipulation/Classes/Abstraites/BPFL_Contrainte.etatPhysiqueDefinir` (`local.liaison`) (make `/Game/Manipulation/Types/S_Contrainte` (`local.transformation`) (`local.axe`) _output_get)))
          (:`NewEnumerator1`
            (goto _label_2))
          (:`NewEnumerator2`
            (goto _label_2))
          (:`NewEnumerator4`
            (`BlueprintMapLibrary.Map_Add` (`local.liaison`) (`local.transformation`) (make `/Game/Manipulation/Types/S_ContraintesAxes` (`/Game/Manipulation/Classes/Abstraites/BPFL_Contrainte.physiqueInverser` (break `/Game/Manipulation/Types/S_ContraintesAxes` _value)) (`/Game/Manipulation/Classes/Abstraites/BPFL_Contrainte.physiqueInverser` (`.y_7_E9BF3B1347812DAA96BB5DA2DA3EA730` (break `/Game/Manipulation/Types/S_ContraintesAxes` _value))) (`/Game/Manipulation/Classes/Abstraites/BPFL_Contrainte.physiqueInverser` (`.z_9_09505AF14F2C322AC4DA548E40D9C07C` (break `/Game/Manipulation/Types/S_ContraintesAxes` _value)))))))
        (else
          (set `local.liaison` _nouvelleliaison_contraintes_2))))
    (:`then_3`
      ; Gestion du composant physique
      (`/Game/Manipulation/Classes/Acteurs/BP_GrapheLiaisons.liaisonNouvelle` _liaisons _piecea _pieceb)
      (`/Game/Manipulation/Classes/Acteurs/BP_GrapheLiaisons.liaisonDecaler` _liaisons _piecea _pieceb (`/Game/Manipulation/Classes/Abstraites/BPFL_Transformation.placementVersTransformation` _nouvelleliaison_placement_3))
      (`/Game/Manipulation/Classes/Acteurs/BP_GrapheLiaisons.liaisonDefinirPhysique` _liaisons _piecea _pieceb (`local.liaison`)))
    (:`then_4`
      ; On vient placer la nouvelle liaison
      (`BlueprintMapLibrary.Map_Add` (`local.pieceLiaisons`) (`local.nomB`) (make `/Game/Manipulation/Types/S_Liaison` (`/Game/Manipulation/Classes/Abstraites/BPFL_Transformation.transformationVersPlacement` (`/Game/Manipulation/Classes/Acteurs/BP_GrapheLiaisons.decalageObtenir` (`self.liaisons`) (`local.pieceA`) (`local.pieceB`))) (`local.liaison`)))
      (`BlueprintMapLibrary.Map_Add` (`local.pieces`) (`local.nomA`) (make `/Game/Manipulation/Types/S_Piece` (`/Game/Manipulation/Classes/Abstraites/BPFL_Transformation.transformationVersPlacement` (`local.pieceTransformation`)) (`local.pieceLiaisons`))))
    (:`then_5`
      ; On écrit notre changement dans la sauvegarde
      (bind _returnvalue_3 (`GameplayStatics.GetActorOfClass` "/Game/Manipulation/Classes/Acteurs/Statiques/BP_Sauvegarde.BP_Sauvegarde_C"))
      (bind _donnees (`/Game/Manipulation/Classes/Acteurs/Statiques/BP_Sauvegarde.lire` _returnvalue_3 self))
      (`/Game/Manipulation/Classes/Acteurs/Statiques/BP_Sauvegarde.ecrire` _returnvalue_3 (make `/Game/Manipulation/Types/S_ChampRobot` (break `/Game/Manipulation/Types/S_ChampRobot` _donnees) (make `/Game/Manipulation/Types/S_Assemblage` (break `/Game/Manipulation/Types/S_Assemblage` (`.assemblage_5_ABD141CF4D373683774A5881ABCE92B3` (break `/Game/Manipulation/Types/S_ChampRobot` _donnees))) (`.placement_7_71A3E01C4139B4D6E77EF5BF3DFF560A` (break `/Game/Manipulation/Types/S_Assemblage` (`.assemblage_5_ABD141CF4D373683774A5881ABCE92B3` (break `/Game/Manipulation/Types/S_ChampRobot` _donnees)))) (`local.pieces`) (`.metadonnees_14_038653E44178F61C1D1BF48AB8B667D2` (break `/Game/Manipulation/Types/S_Assemblage` (`.assemblage_5_ABD141CF4D373683774A5881ABCE92B3` (break `/Game/Manipulation/Types/S_ChampRobot` _donnees))))))))
    (:`then_6`
      ; Affichage console
      (if (`BlueprintMapLibrary.Map_IsEmpty` _nouvelleliaison_contraintes)
        (`/Game/Manipulation/Classes/Abstraites/BPFL_Contrainte.afficher` (make `/Game/Manipulation/Types/S_Contrainte` _transformation _axe (`/Game/Manipulation/Classes/Abstraites/BPFL_Contrainte.etatPhysiqueObtenir` (`local.liaison`) _transformation _axe)) _noma _nomb)
        (else
          (bind _etat (`/Game/Manipulation/Classes/Abstraites/BPML_Contrainte.pourChaqueEtat` (`local.liaison`))
            (:`boucle`
              (`/Game/Manipulation/Classes/Abstraites/BPFL_Contrainte.afficher` _etat _noma _nomb))))))))

(fn `liaisonsChangerActivation`
  (params (aActiver :type Boolean :default true) (attachement :type "EAttachmentRule Enum" :default "KeepWorld"))
  (bind _attachement (`local.attachement`))
  (bind (_arrayindex _arrayelement) (`/Engine/EditorBlueprintResources/StandardMacros.ReverseForEachLoop` (`self.K2_GetComponentsByClass` "/Script/Engine.StaticMeshComponent"))
    (:`LoopBody`
      ; Il faut rattacher les pièces après avoir activé la physique
      (`PrimitiveComponent.SetSimulatePhysics` _arrayelement (`local.aActiver`))
      (`SceneComponent.K2_AttachToComponent` _arrayelement (`self.DefaultSceneRoot`) "None" _attachement _attachement _attachement true))
    (:`Completed`
      ; La base de l'assemblage doit être fixe
      (`PrimitiveComponent.SetSimulatePhysics` (`self.base`) false))))

(fn `liaisonsCharger`
  (locals (pieceA :type "StaticMeshComponent Object Reference") (pieceB :type "StaticMeshComponent Object Reference"))
  (bind _piecea (`local.pieceA`))
  (bind _pieceb (`local.pieceB`))
  (bind _liaisons (`self.liaisons`))
  (bind _returnvalue (`GameplayStatics.GetActorOfClass` "/Game/Manipulation/Classes/Acteurs/Statiques/BP_Sauvegarde.BP_Sauvegarde_C"))
  ; Pour chaque chaque liaison entre deux pièces
  (bind (_keypin _valuepin) (`|MapForEach` (`.pieces_15_AA0EACB64195D6F1CD7D1B8D3DEB6A4A` (break `/Game/Manipulation/Types/S_Assemblage` (`.assemblage_5_ABD141CF4D373683774A5881ABCE92B3` (break `/Game/Manipulation/Types/S_ChampRobot` (`/Game/Manipulation/Classes/Acteurs/Statiques/BP_Sauvegarde.lire` _returnvalue self))))))
    (:`then`
      (set `local.pieceA` (`.piece` (`self.pieceObtenir` _keypin)))
      (bind (_keypin_2 _valuepin_2) (`|MapForEach` (`.liaisons_7_45728FC442F8D33DC8BA7A8E1B036B66` (break `/Game/Manipulation/Types/S_Piece` _valuepin)))
        (:`then`
          (set `local.pieceB` (`.piece` (`self.pieceObtenir` _keypin_2)))
          ; On restaure le placement (x, y, z) de la contrainte
          (`/Game/Manipulation/Classes/Acteurs/BP_GrapheLiaisons.liaisonNouvelle` _liaisons _piecea _pieceb)
          (`/Game/Manipulation/Classes/Acteurs/BP_GrapheLiaisons.liaisonDecaler` _liaisons _piecea _pieceb (`/Game/Manipulation/Classes/Abstraites/BPFL_Transformation.placementVersTransformation` (break `/Game/Manipulation/Types/S_Liaison` _valuepin_2)))
          ; On applique de nouveau chaque type de contrainte
          (`/Game/Manipulation/Classes/Acteurs/BP_GrapheLiaisons.liaisonDefinirPhysique` _liaisons _piecea _pieceb (`.contraintes_7_147DBC5940D797B1F538718E58A09DF9` (break `/Game/Manipulation/Types/S_Liaison` _valuepin_2))))))))

(fn `modeleCharger`
  (locals (nomModele :type String))
  ; Si le robot n'a pas de nom, on ne peut pas charger un modèle pour lui
  (if (not (`KismetStringLibrary.IsEmpty` (`self.nomObtenir`)))
    ; On cherche le fichier dans le dossier des modèles
    (bind _returnvalue (`GameplayStatics.GetActorOfClass` "/Game/Manipulation/Classes/Acteurs/Statiques/BP_Sauvegarde.BP_Sauvegarde_C"))
    (bind _valuepin (`|SetForEach` (`/Game/Manipulation/Classes/Acteurs/Statiques/BP_Sauvegarde.formatsModeles` _returnvalue))
      (:`then`
        (bind _returnvalue_2 (`KismetStringLibrary.Concat_StrStr` (`/Game/Manipulation/Classes/Acteurs/Statiques/BP_Sauvegarde.dossierModeles` _returnvalue) (`self.nomObtenir`) "." _valuepin))
        (bind _returnvalue_3 (`BlueprintFileUtilsBPLibrary.FileExists` _returnvalue_2))
        (if _returnvalue_3
          (set `local.nomModele` _returnvalue_2)))
      (:`CompletedPin`
        (if (`KismetStringLibrary.IsEmpty` (`local.nomModele`))
          ; Erreur : on a rien trouvé, peu importe le format
          (`/Game/Manipulation/Classes/Abstraites/BPFL_Caracteres.erreurAfficher` (`|FormatText` "le modèle \"{nomFichier}\" est introuvable" (`self.nomObtenir`)))
          (else
            (bind _returnvalue_4 (`GameplayStatics.GetActorOfClass` "/Game/Manipulation/Classes/Acteurs/Statiques/BP_Logiciel.BP_Logiciel_C"))
            (bind _tailleutilisateur (`/Game/Manipulation/Classes/Acteurs/Statiques/BP_Logiciel.tailleUtilisateur` _returnvalue_4))
            (if (<= _tailleutilisateur 0.0)
              (`/Game/Manipulation/Classes/Abstraites/BPFL_Caracteres.erreurAfficher` "taille négative")
              (else
                ; On modélise les pièces et les liaisons, mais seules les pièces sont contenues dans les fichiers .glb
                (bind _returnvalue_5 (`glTFRuntimeFunctionLibrary.glTFLoadAssetFromFilename` (`local.nomModele`) false (make `glTFRuntimeConfig` "Default" (struct :`XPlane` (struct :`X` 1.0) :`YPlane` (struct :`Y` 1.0) :`ZPlane` (struct :`Z` 1.0) :`WPlane` (struct :`W` 1.0)) "0.000000,0.000000,0.000000|0.000000,0.000000,-0.000000|1.000000,1.000000,1.000000" (struct :`XAxis` (0.0 0.0 0.0) :`YAxis` (0.0 0.0 0.0) :`ZAxis` (0.0 0.0 0.0) :`Origin` (0.0 0.0 0.0)) _tailleutilisateur)))
                (`self.modeliser` _returnvalue_5)
                (bind _returnvalue_6 (`|SpawnActorFromClass` "/Game/Manipulation/Classes/Acteurs/BP_GrapheLiaisons.BP_GrapheLiaisons_C" (`self.GetTransform`) "Undefined" "MultiplyWithRoot" null self null))
                (set `self.liaisons` _returnvalue_6)))))))))

(fn `modeliser`
  (params (modele :type "glTFRuntimeAsset Object Reference"))
  (locals (maillageIndex :type Integer) (pieceIndex :type Integer) (pieceNouvelle :type "StaticMeshComponent Object Reference") (noeudNom :type String) (occurences :type "Map of String to Object Object Reference") (noeudTransformation :type "Transform Structure" :default "0.000000,0.000000,0.000000|0.000000,0.000000,0.000000|1.000000,1.000000,1.000000"))
  (bind _occurences (`local.occurences`))
  (bind _noeudnom (`local.noeudNom`))
  (bind _value (`BlueprintMapLibrary.Map_Find` _occurences (`local.noeudNom`)))
  (bind (_arrayindex _arrayelement) (`/Engine/EditorBlueprintResources/StandardMacros.ReverseForEachLoop` (`glTFRuntimeAsset.GetNodes` modele))
    (:`LoopBody`
      (set `local.pieceIndex` (break `glTFRuntimeNode` _arrayelement))
      (set `local.noeudNom` (`.Name` (break `glTFRuntimeNode` _arrayelement)))
      ; Si l'index vaut -1, c'est que le noeud ne contient pas de maillage
      (bind _output_get (set `local.maillageIndex` (`.MeshIndex` (break `glTFRuntimeNode` _arrayelement))))
      (if (!= _output_get -1)
        (`|ExecutionSequence`
          (:`then_0`
            ; Chargement du placement du modèle 3D et de ses ancêtres
            (set `local.noeudTransformation` (`self.noeudTransformationGlobale` (`local.pieceIndex`) (`glTFRuntimeAsset.GetNodes` (`local.modele`)))))
          (:`then_1`
            ; On remplace le placement par celui de la sauvegarde, s'il existe
            (bind _returnvalue (`GameplayStatics.GetActorOfClass` "/Game/Manipulation/Classes/Acteurs/Statiques/BP_Sauvegarde.BP_Sauvegarde_C"))
            (bind (_value_2 _returnvalue_2) (`BlueprintMapLibrary.Map_Find` (`.pieces_15_AA0EACB64195D6F1CD7D1B8D3DEB6A4A` (break `/Game/Manipulation/Types/S_Assemblage` (`.assemblage_5_ABD141CF4D373683774A5881ABCE92B3` (break `/Game/Manipulation/Types/S_ChampRobot` (`/Game/Manipulation/Classes/Acteurs/Statiques/BP_Sauvegarde.lire` _returnvalue self))))) (`local.noeudNom`)))
            (if _returnvalue_2
              (set `local.noeudTransformation` (`/Game/Manipulation/Classes/Abstraites/BPFL_Transformation.placementVersTransformation` (break `/Game/Manipulation/Types/S_Piece` _value_2)))))
          (:`then_2`
            ; Nouvelle pièce
            (bind _returnvalue_3 (`AddComponent|NODE_AddStaticMeshComponent-1` :`bManualAttachment` true :`RelativeTransform` (`local.noeudTransformation`)))
            (set `local.pieceNouvelle` _returnvalue_3))
          (:`then_3`
            ; On incorpore le maillage dans le composant
            (bind _returnvalue_4 (`glTFRuntimeAsset.LoadStaticMesh` (`local.modele`) (`local.maillageIndex`) (make `glTFRuntimeStaticMeshConfig` "ReadWrite" false true true _ _ "CTF_UseDefault" true "Asset" (`local.pieceNouvelle`))))
            (`StaticMeshComponent.SetStaticMesh` (`local.pieceNouvelle`) _returnvalue_4))
          (:`then_4`
            ; Si plusieurs pièces ont le même nom, on les numérote
            (`BlueprintMapLibrary.Map_Add` _occurences (`local.noeudNom`) (+ _value 1))
            (switch `int` _value
              (:`Default`
                (`/Game/Manipulation/Classes/Abstraites/BPFL_Piece.nomChanger` (`/Game/Manipulation/Classes/Abstraites/BPFL_Caracteres.numeroAjouter` _value (`local.noeudNom`)) (`local.pieceNouvelle`) :!label _label))
              (:`0`
                (`/Game/Manipulation/Classes/Abstraites/BPFL_Caracteres.erreurAfficher` "nombre négatif d'occurences"))
              (:`1`
                (`/Game/Manipulation/Classes/Abstraites/BPFL_Piece.nomChanger` (`local.noeudNom`) (`local.pieceNouvelle`)))
              (:`2`
                (`|ExecutionSequence`
                  (:`then_0`
                    (`/Game/Manipulation/Classes/Abstraites/BPFL_Piece.nomChanger` (`/Game/Manipulation/Classes/Abstraites/BPFL_Caracteres.numeroAjouter` 1 _noeudnom) (`.piece` (`self.pieceObtenir` _noeudnom))))
                  (:`then_1`
                    (goto _label)))))))))
    (:`Completed`
      ; La base de l'assemblage se comporte différemment
      (set `self.base` (`local.pieceNouvelle`))
      (`self.liaisonsChangerActivation` true "KeepRelative"))))

(fn `moteursStopper`
  (locals (pieceA :type "StaticMeshComponent Object Reference"))
  (bind _liaisons (`self.liaisons`))
  ; On parcourt toutes les liaisons du robot
  (bind _returnvalue (`GameplayStatics.GetActorOfClass` "/Game/Manipulation/Classes/Acteurs/Statiques/BP_Sauvegarde.BP_Sauvegarde_C"))
  (bind (_keypin _valuepin) (`|MapForEach` (`.pieces_15_AA0EACB64195D6F1CD7D1B8D3DEB6A4A` (break `/Game/Manipulation/Types/S_Assemblage` (`.assemblage_5_ABD141CF4D373683774A5881ABCE92B3` (break `/Game/Manipulation/Types/S_ChampRobot` (`/Game/Manipulation/Classes/Acteurs/Statiques/BP_Sauvegarde.lire` _returnvalue self))))))
    (:`then`
      (set `local.pieceA` (`.piece` (`self.pieceObtenir` _keypin)))
      (bind _keypin_2 (`|MapForEach` (`.liaisons_7_45728FC442F8D33DC8BA7A8E1B036B66` (break `/Game/Manipulation/Types/S_Piece` _valuepin)))
        (:`then`
          (`/Game/Manipulation/Classes/Acteurs/BP_GrapheLiaisons.moteurActivation` _liaisons (`/Game/Manipulation/Classes/Acteurs/BP_GrapheLiaisons.composantObtenir` _liaisons (`local.pieceA`) (`.piece` (`self.pieceObtenir` _keypin_2))) false))))))

(fn `noeudTransformationGlobale`
  (params (indexDepart :type Integer) (arbre :type "Array of glTFRuntimeNode Structure"))
  (returns (transformationGlobale :type "Transform Structure"))
  (locals (arbreParcouru :type Boolean :default true) (noeudIndex :type Integer) (transformation :type "Transform Structure"))
  (bind _transformation (`local.transformation`))
  (bind (_output_index _output_name _output_transform _output_meshindex _output_skinindex _output_cameraindex _output_childrenindices _output_parentindex) (break `glTFRuntimeNode` (`|GetArrayItem` arbre (`local.noeudIndex`))))
  ; On va jusqu'à la racine de l'arbre des maillages pour cummuler les transformations
  (set `local.noeudIndex` indexDepart)
  (while (`local.arbreParcouru`)
    (set `local.transformation` (`KismetMathLibrary.ComposeTransforms` _transformation _output_transform))
    (bind _output_get (set `local.noeudIndex` _output_parentindex))
    (set `local.arbreParcouru` (!= _output_get -1)))
  (return _transformation))

(fn `nomObtenir`
  (returns (nom :type String))
  (return (`KismetStringLibrary.Conv_NameToString` (`|GetArrayItem` (`self.Tags`)))))

(fn `pieceObtenir`
  (params (nom :type String))
  (returns (reussite :type Boolean) (piece :type "StaticMeshComponent Object Reference"))
  (bind _returnvalue (`self.GetComponentsByTag` "/Script/Engine.StaticMeshComponent" (`KismetStringLibrary.Conv_StringToName` nom)))
  ; Le tag d'indice 0 est considéré comme le nom de la pièce
  (return (`KismetArrayLibrary.Array_IsNotEmpty` _returnvalue) (`|GetArrayItem` _returnvalue)))

(fn `placementReel`
  (locals (decalages :type "Array of Float (double-precision)") (pieceA :type "StaticMeshComponent Object Reference") (pieceB :type "StaticMeshComponent Object Reference") (decalageLiaison :type "Transform Structure"))
  (bind _decalages (`local.decalages`))
  (bind _returnvalue (`KismetArrayLibrary.Array_LastIndex` _decalages))
  ; On replace le jumeau si le robot réel a bougé, et si cela ne provenait pas d'un jumelage précédent, pour éviter les jumelages à la chaîne
  (bind _returnvalue_2 (`GameplayStatics.GetActorOfClass` "/Game/Manipulation/Classes/Acteurs/Statiques/BP_Requetage.BP_Requetage_C"))
  (bind (_decalages_2 _abouge) (`/Game/Manipulation/Classes/Acteurs/Statiques/BP_Requetage.placementsLire` _returnvalue_2))
  (set `local.decalages` _decalages_2)
  (if _abouge
    (bind _returnvalue_3 (`GameplayStatics.GetActorOfClass` "/Game/Manipulation/Classes/Acteurs/Statiques/BP_Logiciel.BP_Logiciel_C"))
    (switch `/Game/Manipulation/Enumérateurs/E_Jumelage` (`/Game/Manipulation/Classes/Acteurs/Statiques/BP_Logiciel.jumelage` _returnvalue_3)
      (:`NewEnumerator0`
        ; On parcourt toutes les liaisons du robot
        (`KismetArrayLibrary.Array_Reverse` (`local.decalages`) :!label _label)
        (bind _returnvalue_4 (`GameplayStatics.GetActorOfClass` "/Game/Manipulation/Classes/Acteurs/Statiques/BP_Sauvegarde.BP_Sauvegarde_C"))
        (bind (_keypin _valuepin) (`|MapForEach` (`.pieces_15_AA0EACB64195D6F1CD7D1B8D3DEB6A4A` (break `/Game/Manipulation/Types/S_Assemblage` (`.assemblage_5_ABD141CF4D373683774A5881ABCE92B3` (break `/Game/Manipulation/Types/S_ChampRobot` (`/Game/Manipulation/Classes/Acteurs/Statiques/BP_Sauvegarde.lire` _returnvalue_4 self))))))
          (:`then`
            (set `local.pieceA` (`.piece` (`self.pieceObtenir` _keypin)))
            (bind (_keypin_2 _valuepin_2) (`|MapForEach` (`.liaisons_7_45728FC442F8D33DC8BA7A8E1B036B66` (break `/Game/Manipulation/Types/S_Piece` _valuepin)))
              (:`then`
                (set `local.decalageLiaison` (struct))
                (set `local.pieceB` (`.piece` (`self.pieceObtenir` _keypin_2)))
                (bind _etat (`/Game/Manipulation/Classes/Abstraites/BPML_Contrainte.pourChaqueEtat` (`.contraintes_7_147DBC5940D797B1F538718E58A09DF9` (break `/Game/Manipulation/Types/S_Liaison` _valuepin_2)))
                  (:`fin`
                    ; On applique le décalage sur les degrés de liberté de la liaison
                    (`/Game/Manipulation/Classes/Acteurs/BP_GrapheLiaisons.moteurBouger` (`self.liaisons`) (`local.pieceA`) (`local.pieceB`) (`local.decalageLiaison`)))
                  (:`boucle`
                    ; On récupère les décalages de chaque degré de liberté
                    (switch `/Game/Manipulation/Enumérateurs/E_Physique` (break `/Game/Manipulation/Types/S_Physique` (`.physique_9_6356AE914CF5DA94CF165AA84A44D1BA` (break `/Game/Manipulation/Types/S_Contrainte` _etat)))
                      (:`NewEnumerator0`
                        _)
                      (:`NewEnumerator1`
                        _))
                    (set `local.decalageLiaison` (`/Game/Manipulation/Classes/Abstraites/BPFL_Transformation.composanteDefinir` (`local.decalageLiaison`) (`|GetArrayItem` _decalages _returnvalue) (break `/Game/Manipulation/Types/S_Contrainte` _etat) (`.axe_7_BF3857B14A3C2C2C5F9E5E99CA4A2D8B` (break `/Game/Manipulation/Types/S_Contrainte` _etat))))
                    (`KismetArrayLibrary.Array_Remove` (`local.decalages`) _returnvalue))))))))
      (:`NewEnumerator1`
        (set `/Game/Manipulation/Classes/Acteurs/Statiques/BP_Logiciel.jumelage` "NewEnumerator2" _returnvalue_3))
      (:`NewEnumerator4`
        (set `/Game/Manipulation/Classes/Acteurs/Statiques/BP_Logiciel.jumelage` "NewEnumerator0" _returnvalue_3)
        (goto _label)))
    (else
      (bind _returnvalue_5 (`GameplayStatics.GetActorOfClass` "/Game/Manipulation/Classes/Acteurs/Statiques/BP_Logiciel.BP_Logiciel_C"))
      (switch `/Game/Manipulation/Enumérateurs/E_Jumelage` (`/Game/Manipulation/Classes/Acteurs/Statiques/BP_Logiciel.jumelage` _returnvalue_5)
        (:`NewEnumerator2`
          (set `/Game/Manipulation/Classes/Acteurs/Statiques/BP_Logiciel.jumelage` "NewEnumerator4" _returnvalue_5))))))

(fn `renommer`
  (params (nouveauNom :type String))
  (locals (ancienNom :type String) (dossierModeles :type String))
  (`|ExecutionSequence`
    (:`then_0`
      ; On renomme le fichier contenant le modèle 3D
      (bind _returnvalue (`GameplayStatics.GetActorOfClass` "/Game/Manipulation/Classes/Acteurs/Statiques/BP_Sauvegarde.BP_Sauvegarde_C"))
      (set `local.dossierModeles` (`/Game/Manipulation/Classes/Acteurs/Statiques/BP_Sauvegarde.dossierModeles` _returnvalue))
      (bind _donnees (`/Game/Manipulation/Classes/Acteurs/Statiques/BP_Sauvegarde.lire` _returnvalue self))
      (set `local.ancienNom` (break `/Game/Manipulation/Types/S_ChampRobot` _donnees))
      (bind _returnvalue_2 (`KismetStringLibrary.Concat_StrStr` (`local.dossierModeles`) (`BlueprintPathsLibrary.SetExtension` (`local.ancienNom`) (break `/Game/Manipulation/Types/S_Assemblage` (`.assemblage_5_ABD141CF4D373683774A5881ABCE92B3` (break `/Game/Manipulation/Types/S_ChampRobot` _donnees))))))
      (`BlueprintFileUtilsBPLibrary.CopyFile` (`KismetStringLibrary.Concat_StrStr` (`local.dossierModeles`) (`BlueprintPathsLibrary.SetExtension` (`local.nouveauNom`) (break `/Game/Manipulation/Types/S_Assemblage` (`.assemblage_5_ABD141CF4D373683774A5881ABCE92B3` (break `/Game/Manipulation/Types/S_ChampRobot` _donnees))))) _returnvalue_2 false true)
      (`BlueprintFileUtilsBPLibrary.DeleteFile` _returnvalue_2 true true))
    (:`then_1`
      ; Puis, on change l'identifiant dans la sauvegarde Json
      (bind _returnvalue_3 (`GameplayStatics.GetActorOfClass` "/Game/Manipulation/Classes/Acteurs/Statiques/BP_Sauvegarde.BP_Sauvegarde_C"))
      (bind (_donnees_identifiant _donnees_assemblage) (break `/Game/Manipulation/Types/S_ChampRobot` (`/Game/Manipulation/Classes/Acteurs/Statiques/BP_Sauvegarde.lire` _returnvalue_3 self)))
      (`/Game/Manipulation/Classes/Acteurs/Statiques/BP_Sauvegarde.ecrire` _returnvalue_3 (make `/Game/Manipulation/Types/S_ChampRobot` (`local.nouveauNom`) _donnees_assemblage))
      (`/Game/Manipulation/Classes/Acteurs/Statiques/BP_Sauvegarde.identifiantEcrireSuppression` _returnvalue_3 _donnees_identifiant))
    (:`then_2`
      (set `self.Tags` (`|MakeArray` (`KismetStringLibrary.Conv_StringToName` nouveauNom))))))

(fn `selectionDefinir`
  (params (aSelectionner :type Boolean) (organe :type "SceneComponent Object Reference"))
  (`|ExecutionSequence`
    (:`then_0`
      ; Mise à jour des attributs
      (if (`local.aSelectionner`)
        (bind _returnvalue (`GameplayStatics.GetActorOfClass` "/Game/Manipulation/Classes/Acteurs/Statiques/BP_Logiciel.BP_Logiciel_C"))
        (set `/Game/Manipulation/Classes/Acteurs/Statiques/BP_Logiciel.organeSelectionne` (`local.organe`) _returnvalue)
        (else
          (bind _returnvalue_2 (`GameplayStatics.GetActorOfClass` "/Game/Manipulation/Classes/Acteurs/Statiques/BP_Logiciel.BP_Logiciel_C"))
          (set `/Game/Manipulation/Classes/Acteurs/Statiques/BP_Logiciel.organeSelectionne` null _returnvalue_2))))
    (:`then_1`
      (if (`local.aSelectionner`)
        ; On a cliqué sur l'organe (assemblage ou pièce)
        (`|ExecutionSequence`
          (:`then_0`
            (`/Game/Manipulation/Classes/Abstraites/BPFL_Piece.surlignageMettre` true 1.6 (`/Game/Manipulation/Classes/Abstraites/BPFL_Couleur.rouge`) (`local.organe`))
            (bind _returnvalue_3 (`GameplayStatics.GetActorOfClass` "/Game/Manipulation/Classes/Acteurs/Statiques/BP_Logiciel.BP_Logiciel_C"))
            (`/Game/Manipulation/Classes/Acteurs/Statiques/Axes/BP_Transformateur.activationChanger` (`/Game/Manipulation/Classes/Acteurs/Statiques/BP_Logiciel.transformateur` _returnvalue_3) true (`local.organe`))
            (bind _returnvalue_4 (`GameplayStatics.GetActorOfClass` "/Game/Manipulation/Classes/Acteurs/Statiques/BP_Requetage.BP_Requetage_C"))
            (`/Game/Manipulation/Classes/Acteurs/Statiques/BP_Requetage.robotConnecter` _returnvalue_4 self))
          (:`then_1`
            ; Si l'on a sélectionné une pièce, il faut aussi surligner toutes ses pièces liées
            (bind _asstatic_mesh_component (cast `StaticMeshComponent` (`local.organe`)))
            (bind _keypin (`|MapForEach` (break `/Game/Manipulation/Types/S_PiecesLiees` (`BlueprintMapLibrary.Map_Find` (`/Game/Manipulation/Classes/Acteurs/BP_GrapheLiaisons.adjacences` (`self.liaisons`)) _asstatic_mesh_component)))
              (:`then`
                (`/Game/Manipulation/Classes/Abstraites/BPFL_Piece.surlignageMettre` true 1.0 (`/Game/Manipulation/Classes/Abstraites/BPFL_Couleur.bleu`) _keypin)))))
        (else
          ; On a cliqué en dehors de l'organe (assemblage ou pièce)
          (`|ExecutionSequence`
            (:`then_0`
              (`/Game/Manipulation/Classes/Abstraites/BPFL_Piece.surlignageMettre` false 1.0 (struct :`R` 1.0 :`G` 1.0 :`B` 1.0 :`A` 1.0) (`local.organe`))
              (bind _returnvalue_5 (`GameplayStatics.GetActorOfClass` "/Game/Manipulation/Classes/Acteurs/Statiques/BP_Logiciel.BP_Logiciel_C"))
              (`/Game/Manipulation/Classes/Acteurs/Statiques/Axes/BP_Transformateur.activationChanger` (`/Game/Manipulation/Classes/Acteurs/Statiques/BP_Logiciel.transformateur` _returnvalue_5) false (`local.organe`))
              (`self.moteursStopper`))
            (:`then_1`
              ; Si l'on a désélectionné une pièce, il faut aussi enlever le surlignage de toutes ses pièces liées
              (bind _asstatic_mesh_component_2 (cast `StaticMeshComponent` (`local.organe`)))
              (bind _keypin_2 (`|MapForEach` (break `/Game/Manipulation/Types/S_PiecesLiees` (`BlueprintMapLibrary.Map_Find` (`/Game/Manipulation/Classes/Acteurs/BP_GrapheLiaisons.adjacences` (`self.liaisons`)) _asstatic_mesh_component_2)))
                (:`then`
                  (`/Game/Manipulation/Classes/Abstraites/BPFL_Piece.surlignageMettre` false 1.0 (struct :`R` 1.0 :`G` 1.0 :`B` 1.0 :`A` 1.0) _keypin_2))))))))
    (:`then_2`
      ; Affichage console
      (`KismetSystemLibrary.PrintText` (`|FormatText` "{robot} désélectionné" (`self.nomObtenir`)) true true (`/Game/Manipulation/Classes/Abstraites/BPFL_Couleur.rouge`) 10.0))))

(fn `survolDefinir`
  (params (aSurvoler :type Boolean) (organeTouche :type "SceneComponent Object Reference"))
  (locals (organe :type "SceneComponent Object Reference"))
  ; En mode assemblages, ça ne fait pas sens de survoler précisément une pièce
  (bind _returnvalue (`GameplayStatics.GetActorOfClass` "/Game/Manipulation/Classes/Acteurs/Statiques/BP_Logiciel.BP_Logiciel_C"))
  (switch `/Game/Manipulation/Enumérateurs/E_Etat` (`/Game/Manipulation/Classes/Acteurs/Statiques/BP_Logiciel.etat` _returnvalue)
    (:`NewEnumerator0`
      (set `local.organe` (`self.DefaultSceneRoot`)))
    (:`NewEnumerator3`
      (set `local.organe` (`local.organeTouche`) :!label _label))
    (:`NewEnumerator2`
      (goto _label)))
  (`|ExecutionSequence`
    (:`then_0`
      ; Mise à jour des attributs
      (if (`local.aSurvoler`)
        (bind _returnvalue_2 (`GameplayStatics.GetActorOfClass` "/Game/Manipulation/Classes/Acteurs/Statiques/BP_Logiciel.BP_Logiciel_C"))
        (set `/Game/Manipulation/Classes/Acteurs/Statiques/BP_Logiciel.organeSurvole` (`local.organe`) _returnvalue_2)
        (else
          (bind _returnvalue_3 (`GameplayStatics.GetActorOfClass` "/Game/Manipulation/Classes/Acteurs/Statiques/BP_Logiciel.BP_Logiciel_C"))
          (set `/Game/Manipulation/Classes/Acteurs/Statiques/BP_Logiciel.organeSurvole` null _returnvalue_3))))
    (:`then_1`
      ; Voir le graphe d'états
      (if (not (`self.estSelectionneOuLie` (`local.organe`)))
        (`/Game/Manipulation/Classes/Abstraites/BPFL_Piece.surlignageMettre` (`local.aSurvoler`) 1.0 (`/Game/Manipulation/Classes/Abstraites/BPFL_Couleur.jaune`) (`local.organe`))))
    (:`then_2`
      ; Affichage console
      (`KismetSystemLibrary.PrintText` (`|FormatText` "{robot} plus survolé" (`self.nomObtenir`)) true true (`/Game/Manipulation/Classes/Abstraites/BPFL_Couleur.bleuMarine`) 10.0))))

(fn `UserConstructionScript`)