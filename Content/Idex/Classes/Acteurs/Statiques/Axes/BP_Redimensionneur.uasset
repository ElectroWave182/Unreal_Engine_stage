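; BP_Redimensionneur is a scale gizmo that resizes robot parts or assemblies along X, Y, Z or all axes.
; Anchoring stores starting scale, cursor hit and drag direction.
; Dragging projects the cursor ray onto that direction, applying the distance ratio as scale to the target and handle bar, keeping the grabbed point under the cursor.
; Activation disables robot mechanical links; releasing resets the bar and refreshes the selected assembly's links.
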(fn `activationChanger`
  (params (aActiver :type Boolean) (organeTransforme :type "SceneComponent Object Reference"))
  (`parent.activationChanger` aActiver organeTransforme)
  ; Les liaisons mécaniques ne doivent pas intervenir dans la mise à l'échelle
  (`/Game/Idex/Classes/Acteurs/BP_Robot.liaisonsChangerActivation` (cast `/Game/Idex/Classes/Acteurs/BP_Robot` (`ActorComponent.GetOwner` organeTransforme) :!pure true) (not (`local.aActiver`)) "KeepWorld"))

(fn `ancrageChanger`
  (params (organeAncre :type "SceneComponent Object Reference"))
  (`parent.ancrageChanger` organeAncre)
  (switch `/Game/Idex/Enumérateurs/E_Axe` (`self.axeUtilise`)
    (:`NewEnumerator0`
      _)
    (:`NewEnumerator1`
      _)
    (:`NewEnumerator2`
      _)
    (:`NewEnumerator4`
      _))
  (`|ExecutionSequence`
    (:`then_0`
      ; On retient la dimension de départ de l'organe pour pouvoir la comparer ensuite
      (set `self.departOrgane` (`SceneComponent.K2_GetComponentScale` (`local.organeAncre`))))
    (:`then_1`
      ; Position de départ du curseur
      (bind _returnvalue (`GameplayStatics.GetActorOfClass` "/Game/Idex/Classes/Acteurs/Statiques/BP_Personnage.BP_Personnage_C"))
      (set `self.departTirage` (`/Game/Idex/Classes/Acteurs/Statiques/BP_Personnage.curseurCollision` _returnvalue "TraceTypeQuery3")))
    (:`then_2`
      ; Axe d'ajustement
      (set `self.direction` (select `/Game/Idex/Enumérateurs/E_Axe` (`self.axeUtilise`) :`NewEnumerator0` (`self.GetActorForwardVector`) :`NewEnumerator1` (`self.GetActorRightVector`) :`NewEnumerator2` (`self.GetActorUpVector`) :`NewEnumerator4` (`KismetMathLibrary.Normal` (- (`self.departTirage`) (`self.K2_GetActorLocation`))))))
    (:`then_3`
      ; On retient les dimensions pour pouvoir les réinitialiser après un changement visuel
      (set `self.departBarreVisuelle` (`SceneComponent.RelativeScale3D` (`self.indicateurObtenir` (`self.axeUtilise`)))))))

(fn `axesInitialiser`
  (`parent.axesInitialiser`)
  (`|ExecutionSequence`
    (:`then_0`
      (`BlueprintMapLibrary.Map_Add` (`self.axes`) (`self.poigneeX`) "NewEnumerator0"))
    (:`then_1`
      (`BlueprintMapLibrary.Map_Add` (`self.axes`) (`self.poigneeY`) "NewEnumerator1"))
    (:`then_2`
      (`BlueprintMapLibrary.Map_Add` (`self.axes`) (`self.poigneeZ`) "NewEnumerator2"))))

(fn `indicateurObtenir`
  (params (axe :type "/Game/Idex/Enumérateurs/E_Axe Enum" :default "NewEnumerator0"))
  (returns (indicateurVisuel :type "SceneComponent Object Reference"))
  (return (select `/Game/Idex/Enumérateurs/E_Axe` axe :`NewEnumerator0` (`self.barreX`) :`NewEnumerator1` (`self.barreY`) :`NewEnumerator2` (`self.barreZ`) :`NewEnumerator4` (`self.DefaultSceneRoot`) :!type "SceneComponent Object Reference")))

(fn `lier`
  (returns (axe :type "/Game/Idex/Enumérateurs/E_Axe Enum"))
  ; Il n'y a pas de liaison d'échelles
  (return "NewEnumerator3"))

(fn `lierStop`
  (returns (assemblage :type "/Game/Idex/Classes/Acteurs/BP_Robot Object Reference") (pieceA :type "StaticMeshComponent Object Reference") (pieceB :type "StaticMeshComponent Object Reference"))
  ; Il n'y a pas de liaison d'échelles
  (return null null null))

(fn `organeAjustement`
  (returns (ajustement :type "Float (double-precision)"))
  (locals (actuelTirage :type "Vector Structure"))
  (bind _returnvalue (`self.K2_GetActorLocation`))
  ; On cherche le point le plus proche de la demi-droite du pointeur souris
  (`|ExecutionSequence`
    (:`then_0`
      (bind _returnvalue_2 (`GameplayStatics.GetActorOfClass` "/Game/Idex/Classes/Acteurs/Statiques/BP_Personnage.BP_Personnage_C"))
      (bind (_position _direction) (`/Game/Idex/Classes/Acteurs/Statiques/BP_Personnage.curseurPlacement` _returnvalue_2))
      (set `local.actuelTirage` (`.pointD2` (`/Game/Idex/Classes/Abstraites/BPFL_Vecteur.proximiteDroites` _position (`self.departTirage`) _direction (`self.direction`)))))
    (:`then_1`
      ; Le ratio entre le vecteur de tirage actuel et celui de départ nous sert à calculer l'ajutement de la dimension
      (return (/ (`/Game/Idex/Classes/Abstraites/BPFL_Vecteur.distanceSelonAxe` (`self.direction`) (`local.actuelTirage`) _returnvalue) (`/Game/Idex/Classes/Abstraites/BPFL_Vecteur.distanceSelonAxe` (`self.direction`) (`self.departTirage`) _returnvalue))))))

(fn `tirer`
  (returns (organe :type "SceneComponent Object Reference") (axe :type "/Game/Idex/Enumérateurs/E_Axe Enum"))
  (locals (dimensionFin :type "Float (double-precision)") (cible :type "SceneComponent Object Reference"))
  (bind _axeutilise (`self.axeUtilise`))
  ; On tire sur un des trois axes
  (`|ExecutionSequence`
    (:`then_0`
      (bind (_organe _axe) (`parent.tirer`))
      (set `local.cible` _organe)
      (switch `/Game/Idex/Enumérateurs/E_Axe` _axe
        (:`NewEnumerator0`
          _)
        (:`NewEnumerator1`
          _)
        (:`NewEnumerator2`
          _)
        (:`NewEnumerator4`
          _))
      (`|ExecutionSequence`
        (:`then_0`
          ; Le facteur d'ajustement est calculé pour que le curseur de la souris soit toujours sur le même point
          (set `local.dimensionFin` (`self.organeAjustement`)))
        (:`then_1`
          ; On redimensionne l'organe (assemblage ou pièce)
          (`SceneComponent.SetWorldScale3D` (`local.cible`) (`/Game/Idex/Classes/Abstraites/BPFL_Vecteur.composantePonderer` (`self.axeUtilise`) (`local.dimensionFin`) (`self.departOrgane`))))
        (:`then_2`
          ; On déforme aussi la barre tirée pour en faire un repère visuel
          (`SceneComponent.SetRelativeScale3D` (`self.indicateurObtenir` _axeutilise) (`/Game/Idex/Classes/Abstraites/BPFL_Vecteur.composantePonderer` _axeutilise (`local.dimensionFin`) (`self.departBarreVisuelle`))))))
    (:`then_1`
      (return _organe _axe))))

(fn `tirerStop`
  (`|ExecutionSequence`
    (:`then_0`
      ; On remet les dimensions d'origine du repère visuel
      (`SceneComponent.SetRelativeScale3D` (`self.indicateurObtenir` (`self.axeUtilise`)) (`self.departBarreVisuelle`)))
    (:`then_1`
      ; On repositionne les liaisons entre les pièces
      (bind _returnvalue (`GameplayStatics.GetActorOfClass` "/Game/Idex/Classes/Acteurs/Statiques/BP_Logiciel.BP_Logiciel_C"))
      (`/Game/Idex/Classes/Acteurs/BP_GrapheLiaisons.rafraichir` (`/Game/Idex/Classes/Acteurs/BP_Robot.liaisons` (`/Game/Idex/Classes/Acteurs/Statiques/BP_Logiciel.assemblageSelectionne` _returnvalue))))
    (:`then_2`
      (`parent.tirerStop`))))

(fn `UserConstructionScript`)