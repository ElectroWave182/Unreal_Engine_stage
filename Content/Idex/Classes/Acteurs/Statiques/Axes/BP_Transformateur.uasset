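; Transform gizmo actor that snaps onto the selected robot assembly or part for dragging or linking, depending on BP_Logiciel's state.
; Each Tick, a cursor trace resolves the hovered axis through the Axes map, updates robot hover and returns the organ and axis being dragged.
; Releasing a drag saves the transform, calls BP_Requetage and reattaches the gizmo.
; Releasing a link over another part of the same robot highlights it and returns the pair.
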(event `self.ReceiveBeginPlay`
  ; Mise en place
  (`/Game/Idex/Classes/Abstraites/BPFL_Acteur.activationChanger` self)
  (`self.axesInitialiser`))

(event `self.ReceiveTick`
  (params (DeltaSeconds :type "Float (single-precision)"))
  ; Boucle
  (`self.survolRobotChanger` (`self.survolVerifier`))
  (`self.tirer`))

(fn `activationChanger`
  (params (aActiver :type Boolean) (organeTransforme :type "SceneComponent Object Reference"))
  (`|ExecutionSequence`
    (:`then_0`
      ; Récupération de la pièce sélectionnée
      (`self.attachementChanger` (`local.aActiver`) (`local.organeTransforme`)))
    (:`then_1`
      (`/Game/Idex/Classes/Abstraites/BPFL_Acteur.activationChanger` self (`local.aActiver`)))))

(fn `ancrageChanger`
  (params (organeAncre :type "SceneComponent Object Reference"))
  ; Si l'on survole un axe du transformateur, il faut resélectionner l'organe et ancrer le transformateur dessus
  (`/Engine/EditorBlueprintResources/StandardMacros.IsValid` organeAncre
    (:`Is Valid`
      (switch `/Game/Idex/Enumérateurs/E_Axe` (`self.axeSurvole`)
        (:`NewEnumerator0`
          _)
        (:`NewEnumerator1`
          _)
        (:`NewEnumerator2`
          _)
        (:`NewEnumerator4`
          _))
      (`/Game/Idex/Classes/Acteurs/BP_Robot.selectionDefinir` (cast `/Game/Idex/Classes/Acteurs/BP_Robot` (`ActorComponent.GetOwner` organeAncre) :!pure true) true organeAncre)
      (`self.attachementChanger` false)
      (set `self.axeUtilise` (`self.axeSurvole`)))))

(fn `attachementChanger`
  (params (aAttacher :type Boolean) (organe :type "SceneComponent Object Reference"))
  ; On reflète les transformations de l'organe (assemblage ou pièce) sur le transformateur
  (if aAttacher
    (`self.K2_AttachToComponent` (`local.organe`) "None" "SnapToTarget" "SnapToTarget" "KeepWorld")
    (else
      (`self.K2_DetachFromActor` "KeepWorld" "KeepWorld" "KeepWorld"))))

(fn `axesInitialiser`
  (`BlueprintMapLibrary.Map_Add` (`self.axes`) (`self.origine`) "NewEnumerator4"))

(fn `lacher`
  (bind (_estlie _estsurvole _esttire) (`self.utilisation`))
  (if _estlie
    (`self.lierStop`)
    (elif _esttire
      (`self.tirerStop`)))
  (set `self.axeUtilise` "NewEnumerator3"))

(fn `lier`
  (returns (axe :type "/Game/Idex/Enumérateurs/E_Axe Enum"))
  (locals (pieceLiee :type "SceneComponent Object Reference"))
  ; On vérifie qu'on n'est pas en mode assemblages, pièces, ni édition, et qu'une pièce est sélectionnée
  (bind _returnvalue (`GameplayStatics.GetActorOfClass` "/Game/Idex/Classes/Acteurs/Statiques/BP_Logiciel.BP_Logiciel_C"))
  (set `local.pieceLiee` (`/Game/Idex/Classes/Acteurs/Statiques/BP_Logiciel.organeSelectionne` _returnvalue))
  (switch `/Game/Idex/Enumérateurs/E_Etat` (`/Game/Idex/Classes/Acteurs/Statiques/BP_Logiciel.etat` _returnvalue)
    (:`NewEnumerator0`
      _)
    (:`NewEnumerator3`
      (`/Engine/EditorBlueprintResources/StandardMacros.IsValid` (`local.pieceLiee`)
        (:`Is Valid`
          (return (`self.axeUtilise`)))
        (:`Is Not Valid`
          _)))
    (:`NewEnumerator2`
      _)
    (:`NewEnumerator1`
      _)
    (:`NewEnumerator4`
      _))
  (return "NewEnumerator3"))

(fn `lierStop`
  (returns (assemblage :type "/Game/Idex/Classes/Acteurs/BP_Robot Object Reference") (pieceA :type "StaticMeshComponent Object Reference") (pieceB :type "StaticMeshComponent Object Reference"))
  (locals (pieceTouchee :type "SceneComponent Object Reference"))
  (bind _asrobot (cast `/Game/Idex/Classes/Acteurs/BP_Robot` (`ActorComponent.GetOwner` (`local.pieceTouchee`)) :!pure true))
  ; Si on lâche le transformateur sur une autre pièce, on la surligne en bleu
  (bind _returnvalue (`GameplayStatics.GetActorOfClass` "/Game/Idex/Classes/Acteurs/Statiques/BP_Logiciel.BP_Logiciel_C"))
  (bind _organesurvole (`/Game/Idex/Classes/Acteurs/Statiques/BP_Logiciel.organeSurvole` _returnvalue))
  (bind _output_get (set `local.pieceTouchee` _organesurvole))
  (`/Engine/EditorBlueprintResources/StandardMacros.IsValid` _output_get
    (:`Is Valid`
      (bind _organeselectionne (`/Game/Idex/Classes/Acteurs/Statiques/BP_Logiciel.organeSelectionne` _returnvalue))
      (if (and (!= _organesurvole _organeselectionne) (== (cast `/Game/Idex/Classes/Acteurs/BP_Robot` (`ActorComponent.GetOwner` _organeselectionne) :!pure true) _asrobot))
        (`/Game/Idex/Classes/Abstraites/BPFL_Piece.surlignageMettre` true 1.0 (`/Game/Idex/Classes/Abstraites/BPFL_Couleur.bleu`) (`local.pieceTouchee`))
        (return _asrobot (cast `StaticMeshComponent` _organeselectionne :!pure true) (cast `StaticMeshComponent` (`local.pieceTouchee`) :!pure true))))))

(fn `survolRobotChanger`
  (params (axeNouveau :type "/Game/Idex/Enumérateurs/E_Axe Enum" :default "NewEnumerator0"))
  (locals (organeSurvole :type "PrimitiveComponent Object Reference") (assemblageSurvole :type "/Game/Idex/Classes/Acteurs/BP_Robot Object Reference"))
  (bind _organesurvole (`local.organeSurvole`))
  ; On ne continue que si on a survolé un organe différent
  (if (`|EnumInequality` axeNouveau (`self.axeSurvole`))
    (`|ExecutionSequence`
      (:`then_0`
        (set `self.axeSurvole` (`local.axeNouveau`))
        (bind _returnvalue (`GameplayStatics.GetActorOfClass` "/Game/Idex/Classes/Acteurs/Statiques/BP_Personnage.BP_Personnage_C"))
        (set `local.organeSurvole` (`.touche` (`/Game/Idex/Classes/Acteurs/Statiques/BP_Personnage.curseurCollision` _returnvalue "TraceTypeQuery1"))))
      (:`then_1`
        (`/Engine/EditorBlueprintResources/StandardMacros.IsValid` _organesurvole
          (:`Is Valid`
            (bind _asrobot (cast `/Game/Idex/Classes/Acteurs/BP_Robot` (`ActorComponent.GetOwner` _organesurvole)))
            (set `local.assemblageSurvole` _asrobot)
            ; On démarre le survol, ou on le termine selon l'axe précisé
            (switch `/Game/Idex/Enumérateurs/E_Axe` (`self.axeSurvole`)
              (:`NewEnumerator0`
                (`/Game/Idex/Classes/Acteurs/BP_Robot.survolFin` (`local.assemblageSurvole`) (`local.organeSurvole`) :!label _label))
              (:`NewEnumerator1`
                (goto _label))
              (:`NewEnumerator2`
                (goto _label))
              (:`NewEnumerator4`
                (goto _label))
              (:`NewEnumerator3`
                (`/Game/Idex/Classes/Acteurs/BP_Robot.survolDebut` (`local.assemblageSurvole`) (`local.organeSurvole`))))))))))

(fn `survolVerifier`
  (returns (axe :type "/Game/Idex/Enumérateurs/E_Axe Enum"))
  ; On regarde quel axe du transformateur est survolé
  (bind _returnvalue (`GameplayStatics.GetActorOfClass` "/Game/Idex/Classes/Acteurs/Statiques/BP_Logiciel.BP_Logiciel_C"))
  (switch `/Game/Idex/Enumérateurs/E_Etat` (`/Game/Idex/Classes/Acteurs/Statiques/BP_Logiciel.etat` _returnvalue)
    (:`NewEnumerator0`
      _)
    (:`NewEnumerator3`
      _)
    (:`NewEnumerator2`
      _)
    (:`NewEnumerator1`
      (return "NewEnumerator3"))
    (:`NewEnumerator4`
      (return "NewEnumerator3")))
  (bind _returnvalue_2 (`GameplayStatics.GetActorOfClass` "/Game/Idex/Classes/Acteurs/Statiques/BP_Personnage.BP_Personnage_C"))
  (bind (_impact _touche) (`/Game/Idex/Classes/Acteurs/Statiques/BP_Personnage.curseurCollision` _returnvalue_2 "TraceTypeQuery3"))
  (`/Engine/EditorBlueprintResources/StandardMacros.IsValid` _touche
    (:`Is Valid`
      (return (`BlueprintMapLibrary.Map_Find` (`self.axes`) _touche)))
    (:`Is Not Valid`
      (return "NewEnumerator3"))))

(fn `tirer`
  (returns (organe :type "SceneComponent Object Reference") (axe :type "/Game/Idex/Enumérateurs/E_Axe Enum"))
  (locals (organeTire :type "SceneComponent Object Reference"))
  ; On vérifie qu'on n'est pas en mode liaison, ni édition, et qu'un organe (assemblage ou pièce) est sélectionné
  (bind _returnvalue (`GameplayStatics.GetActorOfClass` "/Game/Idex/Classes/Acteurs/Statiques/BP_Logiciel.BP_Logiciel_C"))
  (set `local.organeTire` (`/Game/Idex/Classes/Acteurs/Statiques/BP_Logiciel.organeSelectionne` _returnvalue))
  (switch `/Game/Idex/Enumérateurs/E_Etat` (`/Game/Idex/Classes/Acteurs/Statiques/BP_Logiciel.etat` _returnvalue)
    (:`NewEnumerator0`
      (`/Engine/EditorBlueprintResources/StandardMacros.IsValid` (`local.organeTire`) :!label _label
        (:`Is Valid`
          _)
        (:`Is Not Valid`
          (return (`local.organeTire`) "NewEnumerator3"))))
    (:`NewEnumerator3`
      (return (`local.organeTire`) "NewEnumerator3"))
    (:`NewEnumerator2`
      (goto _label))
    (:`NewEnumerator1`
      (return (`local.organeTire`) "NewEnumerator3"))
    (:`NewEnumerator4`
      (return (`local.organeTire`) "NewEnumerator3")))
  (return (`local.organeTire`) (`self.axeUtilise`)))

(fn `tirerStop`
  (locals (assemblage :type "/Game/Idex/Classes/Acteurs/BP_Robot Object Reference"))
  (`|ExecutionSequence`
    (:`then_0`
      ; Maintenant que le tirage est terminé, on enregistre le mouvement, et on rattache le transformateur à l'organe (assemblage ou pièce)
      (bind _returnvalue (`GameplayStatics.GetActorOfClass` "/Game/Idex/Classes/Acteurs/Statiques/BP_Logiciel.BP_Logiciel_C"))
      (`/Game/Idex/Classes/Acteurs/Statiques/BP_Logiciel.transformationSauvegarder` _returnvalue)
      (bind _returnvalue_2 (`GameplayStatics.GetActorOfClass` "/Game/Idex/Classes/Acteurs/Statiques/BP_Requetage.BP_Requetage_C"))
      (`/Game/Idex/Classes/Acteurs/Statiques/BP_Requetage.robotConnecter` _returnvalue_2 (`/Game/Idex/Classes/Acteurs/Statiques/BP_Logiciel.assemblageSelectionne` _returnvalue))
      (`self.SetActorScale3D` (1.0 1.0 1.0))
      (`self.attachementChanger` true (`/Game/Idex/Classes/Acteurs/Statiques/BP_Logiciel.organeSelectionne` _returnvalue)))
    (:`then_1`
      ; Affichage console
      (bind _returnvalue_3 (`GameplayStatics.GetActorOfClass` "/Game/Idex/Classes/Acteurs/Statiques/BP_Logiciel.BP_Logiciel_C"))
      (`KismetSystemLibrary.PrintText` (`|FormatText` "{robot} transformé" (`/Game/Idex/Classes/Acteurs/BP_Robot.nomObtenir` (`/Game/Idex/Classes/Acteurs/Statiques/BP_Logiciel.assemblageSelectionne` _returnvalue_3))) true true (`/Game/Idex/Classes/Abstraites/BPFL_Couleur.vert`) 10.0))))

(fn `UserConstructionScript`)

(fn `utilisation`
  (returns (estLie :type Boolean) (estSurvole :type Boolean) (estTire :type Boolean))
  (bind _returnvalue (`|EnumInequality` (`self.axeSurvole`) "NewEnumerator3"))
  (bind _returnvalue_2 (`|EnumInequality` (`self.axeUtilise`) "NewEnumerator3"))
  (bind _returnvalue_3 (`GameplayStatics.GetActorOfClass` "/Game/Idex/Classes/Acteurs/Statiques/BP_Logiciel.BP_Logiciel_C"))
  (switch `/Game/Idex/Enumérateurs/E_Etat` (`/Game/Idex/Classes/Acteurs/Statiques/BP_Logiciel.etat` _returnvalue_3)
    (:`NewEnumerator0`
      _)
    (:`NewEnumerator3`
      (return _returnvalue_2 _returnvalue false))
    (:`NewEnumerator2`
      _)
    (:`NewEnumerator1`
      (return false false false))
    (:`NewEnumerator4`
      (return false false false)))
  (return false _returnvalue _returnvalue_2))