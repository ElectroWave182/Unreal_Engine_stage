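; Central manager of a robot digital-twin editor: spawns saved BP_Robot assemblies and shows the VR or desktop interface.
; It tracks hover and selection by edit mode and swaps translate, rotate or scale gizmo actors.
; Tick feeds user distance to highlight materials and detects when the selection stops moving.
; On stop, it saves placements and, depending on twinning state, passes joint offsets to BP_Requetage for the real robot.
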(event `self.ReceiveBeginPlay`
  ; Mise en place
  (`self.initialiserRobots`)
  (`self.transformateurDefinir` "NewEnumerator0")
  (`self.afficherInterface`)
  (`WidgetBlueprintLibrary.SetFocusToGameViewport`))

(event `self.ReceiveTick`
  (params (DeltaSeconds :type "Float (single-precision)"))
  ; Boucle
  (`self.surlignageAdapter`)
  (`self.transformationArret`))

(fn `afficherInterface`
  (locals (transformationComposant :type "Transform Structure" :default "150.000000,0.000000,0.000000|0.000000,180.000000,0.000000|0.100000,0.100000,0.100000"))
  (if (`HeadMountedDisplayFunctionLibrary.IsHeadMountedDisplayEnabled`)
    ; Réalité virtuelle
    (bind _returnvalue (`GameplayStatics.GetActorOfClass` "/Game/Idex/Classes/Acteurs/Statiques/BP_Personnage.BP_Personnage_C"))
    (bind _returnvalue_2 (`AddComponent|NODE_AddWidgetComponent-0` :`self` _returnvalue :`bManualAttachment` true :`RelativeTransform` (`local.transformationComposant`)))
    (`SceneComponent.K2_AttachToComponent` _returnvalue_2 (`/Game/Idex/Classes/Acteurs/Statiques/BP_Personnage.camera` _returnvalue) "None" "KeepRelative" "KeepRelative" "KeepRelative" true)
    (else
      ; Clavier-souris
      (bind _returnvalue_3 (`|CreateWidget` "/Game/Idex/Classes/WB_Interface.WB_Interface_C" (`GameplayStatics.GetPlayerController` 0)))
      (`UserWidget.AddToViewport` _returnvalue_3 0))))

(fn `assemblageExiste`
  (params (nom :type String))
  (returns (existe :type Boolean))
  ; Unreal Engine étant bien fait, il stocke les tags comme clés d'un dictionnaire d'acteurs ; cela permet à cette fonction d'être en complexité constante, grâce à la table de hachage
  (bind _outactors (`GameplayStatics.GetAllActorsOfClassWithTag` "/Game/Idex/Classes/Acteurs/BP_Robot.BP_Robot_C" (`KismetStringLibrary.Conv_StringToName` nom)))
  (return (`KismetArrayLibrary.Array_IsNotEmpty` _outactors)))

(fn `assemblageSelectionne`
  (returns (assemblage :type "/Game/Idex/Classes/Acteurs/BP_Robot Object Reference"))
  (bind _organeselectionne (`self.organeSelectionne`))
  (`/Engine/EditorBlueprintResources/StandardMacros.IsValid` _organeselectionne
    (:`Is Valid`
      (return (cast `/Game/Idex/Classes/Acteurs/BP_Robot` (`ActorComponent.GetOwner` _organeselectionne) :!pure true)))))

(fn `assemblageSurvole`
  (returns (assemblage :type "/Game/Idex/Classes/Acteurs/BP_Robot Object Reference"))
  (bind _organesurvole (`self.organeSurvole`))
  (`/Engine/EditorBlueprintResources/StandardMacros.IsValid` _organesurvole
    (:`Is Valid`
      (return (cast `/Game/Idex/Classes/Acteurs/BP_Robot` (`ActorComponent.GetOwner` _organesurvole) :!pure true)))))

(fn `initialiserRobots`
  (locals (sauvegarde :type "/Game/Idex/Classes/Acteurs/Statiques/BP_Sauvegarde Object Reference"))
  ; On fait apparaitre un robot selon chaque champ présent dans la sauvegarde
  (bind _returnvalue (`GameplayStatics.GetActorOfClass` "/Game/Idex/Classes/Acteurs/Statiques/BP_Sauvegarde.BP_Sauvegarde_C"))
  (bind _output_get (set `local.sauvegarde` _returnvalue))
  (bind _valuepin (`|SetForEach` (`/Game/Idex/Classes/Acteurs/Statiques/BP_Sauvegarde.identifiantsObtenir` _output_get))
    (:`then`
      (bind _donnees (`/Game/Idex/Classes/Acteurs/Statiques/BP_Sauvegarde.identifiantLire` (`local.sauvegarde`) _valuepin))
      (bind _returnvalue_2 (`|SpawnActorFromClass` "/Game/Idex/Classes/Acteurs/BP_Robot.BP_Robot_C" (`/Game/Idex/Classes/Abstraites/BPFL_Transformation.placementVersTransformation` (`.placement_7_71A3E01C4139B4D6E77EF5BF3DFF560A` (break `/Game/Idex/Types/S_Assemblage` (`.assemblage_5_ABD141CF4D373683774A5881ABCE92B3` (break `/Game/Idex/Types/S_ChampRobot` _donnees))))) "Undefined" "MultiplyWithRoot" null (`|MakeArray` (`KismetStringLibrary.Conv_StringToName` (break `/Game/Idex/Types/S_ChampRobot` _donnees))) null))
      (`/Game/Idex/Classes/Acteurs/BP_Robot.liaisonsCharger` _returnvalue_2))))

(fn `selectionNettoyer`
  (returns (organeNettoye :type "SceneComponent Object Reference"))
  (locals (selectionPrecedente :type "SceneComponent Object Reference"))
  (bind _organeselectionne (`self.organeSelectionne`))
  ; Désélectionne l'organe (assemblage ou pièce) sélectionné
  (switch `/Game/Idex/Enumérateurs/E_Etat` (`self.etat`)
    (:`NewEnumerator0`
      _)
    (:`NewEnumerator3`
      _)
    (:`NewEnumerator2`
      _))
  (bind _output_get (set `local.selectionPrecedente` _organeselectionne))
  (`/Engine/EditorBlueprintResources/StandardMacros.IsValid` _output_get
    (:`Is Valid`
      (`/Game/Idex/Classes/Acteurs/BP_Robot.selectionDefinir` (`self.assemblageSelectionne`) false _organeselectionne)
      (return (`local.selectionPrecedente`)))))

(fn `surlignageAdapter`
  (bind (_keypin _valuepin) (`|MapForEach` (`self.surlignages`))
    (:`then`
      (bind _returnvalue (`GameplayStatics.GetActorOfClass` "/Game/Idex/Classes/Acteurs/Statiques/BP_Personnage.BP_Personnage_C"))
      (`MaterialInstanceDynamic.SetScalarParameterValue` _valuepin "distance" (`KismetMathLibrary.Vector_Distance` (`self.K2_GetActorLocation` _returnvalue) (`SceneComponent.K2_GetComponentLocation` _keypin))))))

(fn `survolRemplacer`
  (params (aSuvoler :type "PrimitiveComponent Object Reference"))
  (locals (composantTouche :type "SceneComponent Object Reference") (organeAncien :type "SceneComponent Object Reference"))
  (bind _asuvoler (`local.aSuvoler`))
  (bind _asuvoler_2 (`local.aSuvoler`))
  (bind _organeancien (`local.organeAncien`))
  (`|ExecutionSequence`
    (:`then_0`
      (bind _returnvalue (`GameplayStatics.GetActorOfClass` "BP_Logiciel_C"))
      (set `local.organeAncien` (`/Game/Idex/Classes/Acteurs/Statiques/BP_Logiciel.organeSurvole` _returnvalue)))
    (:`then_1`
      ; Si on a passé le curseur sur du vide ou sur un objet d'un autre type, on considère qu'on a survolé du vide
      (`/Engine/EditorBlueprintResources/StandardMacros.IsValid` _asuvoler
        (:`Is Valid`
          (bind _asrobot (cast `/Game/Idex/Classes/Acteurs/BP_Robot` (`ActorComponent.GetOwner` _asuvoler))
            (:`then`
              ; Sinon, on applique la logique du mode assemblages : considérer le composant racine comme touché
              (switch `/Game/Idex/Enumérateurs/E_Etat` (`self.etat`)
                (:`NewEnumerator0`
                  (set `local.composantTouche` (`/Game/Idex/Classes/Acteurs/BP_Robot.DefaultSceneRoot` _asrobot)))
                (:`NewEnumerator3`
                  (set `local.composantTouche` (`local.aSuvoler`) :!label _label))
                (:`NewEnumerator2`
                  (goto _label))))
            (:`CastFailed`
              (set `local.composantTouche` null :!label _label_2))))
        (:`Is Not Valid`
          (goto _label_2))))
    (:`then_2`
      ; Si le nouvel organe survolé est différent de l'ancien, on effectue le remplacement
      (if (!= (`local.composantTouche`) (`local.organeAncien`))
        (`|ExecutionSequence`
          (:`then_0`
            (`/Engine/EditorBlueprintResources/StandardMacros.IsValid` _organeancien
              (:`Is Valid`
                (`/Game/Idex/Classes/Acteurs/BP_Robot.survolDefinir` (cast `/Game/Idex/Classes/Acteurs/BP_Robot` (`ActorComponent.GetOwner` _organeancien) :!pure true) false _organeancien))))
          (:`then_1`
            (`/Engine/EditorBlueprintResources/StandardMacros.IsValid` _asuvoler_2
              (:`Is Valid`
                (bind _asrobot_2 (cast `/Game/Idex/Classes/Acteurs/BP_Robot` (`ActorComponent.GetOwner` _asuvoler_2)))
                (`/Game/Idex/Classes/Acteurs/BP_Robot.survolDebut` _asrobot_2 _asuvoler_2)))))))))

(fn `transformateurChanger`
  (params (type :type "/Game/Idex/Enumérateurs/E_Transformation Enum" :default "NewEnumerator0"))
  (bind _organeselectionne (`self.organeSelectionne`))
  (bind _transformateur (`self.transformateur`))
  ; On désactive l'ancien transformateur, et on active le nouveau
  (`/Engine/EditorBlueprintResources/StandardMacros.IsValid` (`self.organeSelectionne`)
    (:`Is Valid`
      (`/Game/Idex/Classes/Acteurs/Statiques/Axes/BP_Transformateur.activationChanger` _transformateur false _organeselectionne)
      (`self.transformateurDefinir` (`local.type`))
      (`/Game/Idex/Classes/Acteurs/Statiques/Axes/BP_Transformateur.activationChanger` _transformateur true _organeselectionne))
    (:`Is Not Valid`
      (`self.transformateurDefinir` (`local.type`)))))

(fn `transformateurDefinir`
  (params (type :type "/Game/Idex/Enumérateurs/E_Transformation Enum" :default "NewEnumerator0"))
  (switch `/Game/Idex/Enumérateurs/E_Transformation` type
    (:`NewEnumerator0`
      (bind _returnvalue (`GameplayStatics.GetActorOfClass` "/Game/Idex/Classes/Acteurs/Statiques/Axes/BP_Translateur.BP_Translateur_C"))
      (set `self.transformateur` _returnvalue))
    (:`NewEnumerator1`
      (bind _returnvalue_2 (`GameplayStatics.GetActorOfClass` "/Game/Idex/Classes/Acteurs/Statiques/Axes/BP_Rotateur.BP_Rotateur_C"))
      (set `self.transformateur` _returnvalue_2))
    (:`NewEnumerator2`
      (bind _returnvalue_3 (`GameplayStatics.GetActorOfClass` "/Game/Idex/Classes/Acteurs/Statiques/Axes/BP_Redimensionneur.BP_Redimensionneur_C"))
      (set `self.transformateur` _returnvalue_3))))

(fn `transformationArret`
  (bind _organeselectionne (`self.organeSelectionne`))
  ; On regarde si le mouvement de l'organe (assemblage ou pièce) vient tout juste de cesser
  (`/Engine/EditorBlueprintResources/StandardMacros.IsValid` _organeselectionne
    (:`Is Valid`
      (if (!= (`self.selectionArretee`) (== (0.0 0.0 0.0) (`SceneComponent.GetComponentVelocity` _organeselectionne) :`ErrorTolerance` 1.0))
        (`|ExecutionSequence`
          (:`then_0`
            (set `self.selectionArretee` (not (`self.selectionArretee`))))
          (:`then_1`
            ; Si c'est le cas, on enregistre ce mouvement dans la sauvegarde
            (if (`self.selectionArretee`)
              (`self.transformationSauvegarder`)
              ; On applique le repositionnement sur le véritable robot
              (bind _returnvalue (`GameplayStatics.GetActorOfClass` "/Game/Idex/Classes/Acteurs/Statiques/BP_Requetage.BP_Requetage_C"))
              (`/Game/Idex/Classes/Acteurs/Statiques/BP_Requetage.robotConnecter` _returnvalue (`self.assemblageSelectionne`)))))))))

(fn `transformationSauvegarder`
  (locals (decalages :type "Array of Float (double-precision)") (pieces :type "Map of String to /Game/Idex/Types/S_Piece Structure") (difference :type "Transform Structure") (transformationA :type "Transform Structure") (transformationB :type "Transform Structure"))
  (`|ExecutionSequence`
    (:`then_0`
      (switch `/Game/Idex/Enumérateurs/E_Jumelage` (`self.jumelage`)
        (:`NewEnumerator0`
          (set `self.jumelage` "NewEnumerator2"))
        (:`NewEnumerator2`
          (set `self.jumelage` "NewEnumerator1"))))
    (:`then_1`
      ; On sauvegarde le mouvement de transformation de chaque pièce
      (bind _returnvalue (`GameplayStatics.GetActorOfClass` "/Game/Idex/Classes/Acteurs/Statiques/BP_Sauvegarde.BP_Sauvegarde_C"))
      (bind _output_get (set `local.pieces` (`.pieces_15_AA0EACB64195D6F1CD7D1B8D3DEB6A4A` (break `/Game/Idex/Types/S_Assemblage` (`.assemblage_5_ABD141CF4D373683774A5881ABCE92B3` (break `/Game/Idex/Types/S_ChampRobot` (`/Game/Idex/Classes/Acteurs/Statiques/BP_Sauvegarde.lire` _returnvalue (`self.assemblageSelectionne`))))))))
      (bind (_keypin _valuepin) (`|MapForEach` _output_get)
        (:`then`
          (bind _output_get_2 (set `local.transformationA` (`SceneComponent.GetRelativeTransform` (`.piece` (`/Game/Idex/Classes/Acteurs/BP_Robot.pieceObtenir` (`self.assemblageSelectionne`) _keypin)))))
          (`BlueprintMapLibrary.Map_Add` (`local.pieces`) _keypin (make `/Game/Idex/Types/S_Piece` (`/Game/Idex/Classes/Abstraites/BPFL_Transformation.transformationVersPlacement` _output_get_2) (`.liaisons_7_45728FC442F8D33DC8BA7A8E1B036B66` (break `/Game/Idex/Types/S_Piece` _valuepin))))
          (switch `/Game/Idex/Enumérateurs/E_Jumelage` (`self.jumelage`)
            (:`NewEnumerator1`
              ; On liste également les décalages des degrés de liberté de l'assemblage pour les appliquer sur le vrai robot
              (bind (_keypin_2 _valuepin_2) (`|MapForEach` (`.liaisons_7_45728FC442F8D33DC8BA7A8E1B036B66` (break `/Game/Idex/Types/S_Piece` _valuepin)))
                (:`then`
                  (bind _output_get_3 (set `local.transformationB` (`SceneComponent.GetRelativeTransform` (`.piece` (`/Game/Idex/Classes/Acteurs/BP_Robot.pieceObtenir` (`self.assemblageSelectionne`) _keypin_2)))))
                  (set `local.difference` (`/Game/Idex/Classes/Abstraites/BPFL_Transformation.soustraire` _output_get_3 (`local.transformationA`)))
                  (bind _etat (`/Game/Idex/Classes/Abstraites/BPML_Contrainte.pourChaqueEtat` (`.contraintes_7_147DBC5940D797B1F538718E58A09DF9` (break `/Game/Idex/Types/S_Liaison` _valuepin_2)))
                    (:`boucle`
                      (switch `/Game/Idex/Enumérateurs/E_Physique` (break `/Game/Idex/Types/S_Physique` (`.physique_9_6356AE914CF5DA94CF165AA84A44D1BA` (break `/Game/Idex/Types/S_Contrainte` _etat)))
                        (:`NewEnumerator0`
                          _)
                        (:`NewEnumerator1`
                          _))
                      (`KismetArrayLibrary.Array_Add` (`local.decalages`) (`/Game/Idex/Classes/Abstraites/BPFL_Transformation.composanteObtenir` (`local.difference`) (break `/Game/Idex/Types/S_Contrainte` _etat) (`.axe_7_BF3857B14A3C2C2C5F9E5E99CA4A2D8B` (break `/Game/Idex/Types/S_Contrainte` _etat)))))))))))))
    (:`then_2`
      ; Puis, celui de l'assemblage
      (bind _returnvalue_2 (`GameplayStatics.GetActorOfClass` "/Game/Idex/Classes/Acteurs/Statiques/BP_Sauvegarde.BP_Sauvegarde_C"))
      (bind _donnees (`/Game/Idex/Classes/Acteurs/Statiques/BP_Sauvegarde.lire` _returnvalue_2 (`self.assemblageSelectionne`)))
      (`/Game/Idex/Classes/Acteurs/Statiques/BP_Sauvegarde.ecrire` _returnvalue_2 (make `/Game/Idex/Types/S_ChampRobot` (break `/Game/Idex/Types/S_ChampRobot` _donnees) (make `/Game/Idex/Types/S_Assemblage` (break `/Game/Idex/Types/S_Assemblage` (`.assemblage_5_ABD141CF4D373683774A5881ABCE92B3` (break `/Game/Idex/Types/S_ChampRobot` _donnees))) (`/Game/Idex/Classes/Abstraites/BPFL_Transformation.transformationVersPlacement` (`self.GetTransform` (`self.assemblageSelectionne`))) (`local.pieces`) (`.metadonnees_14_038653E44178F61C1D1BF48AB8B667D2` (break `/Game/Idex/Types/S_Assemblage` (`.assemblage_5_ABD141CF4D373683774A5881ABCE92B3` (break `/Game/Idex/Types/S_ChampRobot` _donnees))))))))
    (:`then_3`
      ; Sauvegarde de la liste des décalages
      (bind _returnvalue_3 (`GameplayStatics.GetActorOfClass` "/Game/Idex/Classes/Acteurs/Statiques/BP_Requetage.BP_Requetage_C"))
      (`/Game/Idex/Classes/Acteurs/Statiques/BP_Requetage.placementsEcrire` _returnvalue_3 (`local.decalages`)))))

(fn `UserConstructionScript`)