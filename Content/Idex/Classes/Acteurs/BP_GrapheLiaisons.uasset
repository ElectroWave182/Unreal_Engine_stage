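; Actor holding the graph of physical links between a robot's static mesh pieces.
; A nested adjacency map stores one physics constraint component per directed pair, with single-piece links stored as self-edges.
; Functions create constraints on the robot, offset them in piece-local axes, apply per-axis linear and angular limits, and rebind them on refresh.
; The reference-frame adjustment for limit centres is flagged in the graph as incorrect.
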(event `self.ReceiveBeginPlay`
  ; Mise en place
  (`self.initialiser`))

(fn `composantAjouter`
  (params (pieceA :type "StaticMeshComponent Object Reference") (pieceB :type "StaticMeshComponent Object Reference") (contrainteComposant :type "PhysicsConstraintComponent Object Reference"))
  (locals (liaisons :type "/Game/Idex/Types/S_PiecesLiees Structure"))
  (bind _liaisons_voisinage (break `/Game/Idex/Types/S_PiecesLiees` (`local.liaisons`)))
  (bind _liaisons_voisinage_2 (break `/Game/Idex/Types/S_PiecesLiees` (`local.liaisons`)))
  (`|ExecutionSequence`
    (:`then_0`
      ; On récupère le graphe par référence simple (non profonde) ; on doit donc passer par une variable provisoire pour effectuer l'affectation profonde
      (set `local.liaisons` (`BlueprintMapLibrary.Map_Find` (`self.adjacences`) (`local.pieceA`))))
    (:`then_1`
      (`/Engine/EditorBlueprintResources/StandardMacros.IsValid` (`local.pieceB`)
        (:`Is Valid`
          (`BlueprintMapLibrary.Map_Add` _liaisons_voisinage_2 (`local.pieceB`) (`local.contrainteComposant`)))
        (:`Is Not Valid`
          ; Si l'on a pas fourni de pièce secondaire, on considère qu'on ajoute une liaison unique
          (`BlueprintMapLibrary.Map_Add` _liaisons_voisinage (`local.pieceA`) (`local.contrainteComposant`)))))
    (:`then_2`
      (`BlueprintMapLibrary.Map_Add` (`self.adjacences`) (`local.pieceA`) (`local.liaisons`)))))

(fn `composantCreer`
  (params (pieceA :type "StaticMeshComponent Object Reference") (pieceB :type "StaticMeshComponent Object Reference"))
  (returns (contrainteComposant :type "PhysicsConstraintComponent Object Reference"))
  ; On crée la contrainte physique
  (bind _returnvalue (`AddComponent|NODE_AddPhysicsConstraintComponent-1` :`self` (`self.robot`) :`bManualAttachment` true :`RelativeTransform` (`KismetMathLibrary.MakeTransform` (`SceneComponent.K2_GetComponentLocation` (`local.pieceB`)) (`SceneComponent.K2_GetComponentRotation` (`local.pieceA`)))))
  (return _returnvalue))

(fn `contrainteCreer`
  (params (pieceA :type "StaticMeshComponent Object Reference") (pieceB :type "StaticMeshComponent Object Reference"))
  (bind _composant (`self.contrainteObtenir` pieceA pieceB))
  (`|ExecutionSequence`
    (:`then_0`
      ; On détruit l'ancien composant
      (`/Engine/EditorBlueprintResources/StandardMacros.IsValid` _composant
        (:`Is Valid`
          (`ActorComponent.K2_DestroyComponent` _composant))))
    (:`then_1`
      ; On crée le composant physique, et on l'ajoute au graphe
      (bind _contraintecomposant (`self.composantCreer` pieceA pieceB))
      (`self.composantAjouter` (`local.pieceA`) (`local.pieceB`) _contraintecomposant))))

(fn `contrainteDecaler`
  (params (pieceA :type "StaticMeshComponent Object Reference") (pieceB :type "StaticMeshComponent Object Reference") (decalage :type "Transform Structure"))
  (locals (composant :type "PhysicsConstraintComponent Object Reference"))
  ; On applique la transformation par dessus l'ancien placement
  (bind _output_get (set `local.composant` (`self.contrainteObtenir` pieceA pieceB)))
  (`SceneComponent.K2_SetRelativeTransform` _output_get (`/Game/Idex/Classes/Abstraites/BPFL_Transformation.additionner` (`KismetMathLibrary.MakeTransform` (`KismetMathLibrary.GreaterGreater_VectorRotator` decalage_Location (`SceneComponent.K2_GetComponentRotation` (`local.pieceB`))) decalage_Rotation decalage_Scale) (`SceneComponent.GetRelativeTransform` (`local.composant`))) false true))

(fn `contrainteNouvelle`
  (params (pieceA :type "StaticMeshComponent Object Reference") (pieceB :type "StaticMeshComponent Object Reference"))
  ; Si la contrainte physique n'existe pas déjà, on la crée
  (`/Engine/EditorBlueprintResources/StandardMacros.IsValid` (`self.contrainteObtenir` pieceA pieceB)
    (:`Is Not Valid`
      (`self.contrainteCreer` (`local.pieceA`) (`local.pieceB`)))))

(fn `contrainteObtenir`
  (params (pieceA :type "StaticMeshComponent Object Reference") (pieceB :type "StaticMeshComponent Object Reference"))
  (returns (composant :type "PhysicsConstraintComponent Object Reference"))
  (bind _value (`BlueprintMapLibrary.Map_Find` (`self.adjacences`) pieceA))
  (`/Engine/EditorBlueprintResources/StandardMacros.IsValid` (`local.pieceB`)
    (:`Is Valid`
      (return (`BlueprintMapLibrary.Map_Find` (break `/Game/Idex/Types/S_PiecesLiees` _value) pieceB)))
    (:`Is Not Valid`
      ; On prend en compte les liaisons unilatérales
      (return (`BlueprintMapLibrary.Map_Find` (break `/Game/Idex/Types/S_PiecesLiees` _value) (`local.pieceA`))))))

(fn `decalageObtenir`
  (params (pieceA :type "StaticMeshComponent Object Reference") (pieceB :type "StaticMeshComponent Object Reference"))
  (returns (decalage :type "Transform Structure"))
  (bind (_difference_location _difference_rotation _difference_scale) (`KismetMathLibrary.BreakTransform` (`/Game/Idex/Classes/Abstraites/BPFL_Transformation.soustraire` (`SceneComponent.GetRelativeTransform` (`self.contrainteObtenir` pieceA pieceB)) (`KismetMathLibrary.MakeTransform` (`SceneComponent.K2_GetComponentLocation` pieceB) (`SceneComponent.K2_GetComponentRotation` (`local.pieceA`))))))
  ; On change le placement en base locale aux deux pièces (A pour la rotation, B pour la translation)
  (return (`KismetMathLibrary.MakeTransform` (`KismetMathLibrary.LessLess_VectorRotator` _difference_location (`SceneComponent.K2_GetComponentRotation` (`local.pieceB`))) _difference_rotation _difference_scale)))

(fn `initialiser`
  ; On intialise les sommets du graphe
  (for _array_element (`self.K2_GetComponentsByClass` (`self.robot`) "/Script/Engine.StaticMeshComponent")
    (`BlueprintMapLibrary.Map_Add` (`self.adjacences`) _array_element)))

(fn `liaisonDefinirPhysique`
  (params (pieceA :type "StaticMeshComponent Object Reference") (pieceB :type "StaticMeshComponent Object Reference") (contraintes :type "Map of /Game/Idex/Enumérateurs/E_Transformation Enum to /Game/Idex/Types/S_ContraintesAxes Structure"))
  (locals (composant :type "PhysicsConstraintComponent Object Reference") (cadreRotation :type "Rotator Structure") (cadreTranslation :type "Vector Structure"))
  (bind _piecea (`local.pieceA`))
  (bind _pieceb (`local.pieceB`))
  (bind _contraintes (`local.contraintes`))
  (bind _value (`BlueprintMapLibrary.Map_Find` _contraintes "NewEnumerator1"))
  (bind _value_2 (`BlueprintMapLibrary.Map_Find` _contraintes "NewEnumerator0"))
  (bind _returnvalue (`SceneComponent.K2_GetComponentToWorld` (`local.pieceA`)))
  (bind _returnvalue_2 (`KismetMathLibrary.MakeRelativeTransform` (`SceneComponent.K2_GetComponentToWorld` (`local.composant`)) _returnvalue))
  (`|ExecutionSequence`
    (:`then_0`
      ; On réajuste la position et l'orientation de la contrainte pour correspondre à l'état actuel des pièces
      (bind _output_get (set `local.composant` (`self.contrainteObtenir` _piecea _pieceb)))
      (`PhysicsConstraintComponent.SetConstrainedComponents` _output_get _piecea "None" _pieceb "None"))
    (:`then_1`
      ; On applique les états physiques des contraintes sur la translation ; pour celle-ci, Unreal Engine n'a qu'une seule valeur limite qui affecte la distance entre les deux pièces contraintes
      (bind _returnvalue_3 (`PhysicsConstraintComponent.GetConstraint` (`local.composant`)))
      (`ConstraintInstanceBlueprintLibrary.SetLinearLimits` _returnvalue_3 (`/Game/Idex/Classes/Abstraites/BPFL_Contrainte.etatPhysiqueLineaire` (break `/Game/Idex/Types/S_Physique` (break `/Game/Idex/Types/S_ContraintesAxes` _value_2))) (`/Game/Idex/Classes/Abstraites/BPFL_Contrainte.etatPhysiqueLineaire` (break `/Game/Idex/Types/S_Physique` (`.y_7_E9BF3B1347812DAA96BB5DA2DA3EA730` (break `/Game/Idex/Types/S_ContraintesAxes` _value_2)))) (`/Game/Idex/Classes/Abstraites/BPFL_Contrainte.etatPhysiqueLineaire` (break `/Game/Idex/Types/S_Physique` (`.z_9_09505AF14F2C322AC4DA548E40D9C07C` (break `/Game/Idex/Types/S_ContraintesAxes` _value_2)))) (`KismetMathLibrary.FMax` (`.limiteAmplitude_6_B89E3C1940B78CDC8FB9638773D52084` (break `/Game/Idex/Types/S_Physique` (break `/Game/Idex/Types/S_ContraintesAxes` _value_2))) (`.limiteAmplitude_6_B89E3C1940B78CDC8FB9638773D52084` (break `/Game/Idex/Types/S_Physique` (`.y_7_E9BF3B1347812DAA96BB5DA2DA3EA730` (break `/Game/Idex/Types/S_ContraintesAxes` _value_2)))) (`.limiteAmplitude_6_B89E3C1940B78CDC8FB9638773D52084` (break `/Game/Idex/Types/S_Physique` (`.z_9_09505AF14F2C322AC4DA548E40D9C07C` (break `/Game/Idex/Types/S_ContraintesAxes` _value_2))))))
      (set `local.cadreTranslation` (`KismetMathLibrary.MakeVector` (`.limiteCentre_7_B143762145DDCD4F0453E6A849C59040` (break `/Game/Idex/Types/S_Physique` (break `/Game/Idex/Types/S_ContraintesAxes` _value_2))) (`.limiteCentre_7_B143762145DDCD4F0453E6A849C59040` (break `/Game/Idex/Types/S_Physique` (`.y_7_E9BF3B1347812DAA96BB5DA2DA3EA730` (break `/Game/Idex/Types/S_ContraintesAxes` _value_2)))) (`.limiteCentre_7_B143762145DDCD4F0453E6A849C59040` (break `/Game/Idex/Types/S_Physique` (`.z_9_09505AF14F2C322AC4DA548E40D9C07C` (break `/Game/Idex/Types/S_ContraintesAxes` _value_2)))))))
    (:`then_2`
      ; On applique les états physiques des contraintes sur la rotation (Swing1 tourne autour de Z, et Twist autour de X)
      (bind _returnvalue_4 (`PhysicsConstraintComponent.GetConstraint` (`local.composant`)))
      (`ConstraintInstanceBlueprintLibrary.SetAngularLimits` _returnvalue_4 (`/Game/Idex/Classes/Abstraites/BPFL_Contrainte.etatPhysiqueAngulaire` (break `/Game/Idex/Types/S_Physique` (`.z_9_09505AF14F2C322AC4DA548E40D9C07C` (break `/Game/Idex/Types/S_ContraintesAxes` _value)))) (`.limiteAmplitude_6_B89E3C1940B78CDC8FB9638773D52084` (break `/Game/Idex/Types/S_Physique` (`.z_9_09505AF14F2C322AC4DA548E40D9C07C` (break `/Game/Idex/Types/S_ContraintesAxes` _value)))) (`/Game/Idex/Classes/Abstraites/BPFL_Contrainte.etatPhysiqueAngulaire` (break `/Game/Idex/Types/S_Physique` (`.y_7_E9BF3B1347812DAA96BB5DA2DA3EA730` (break `/Game/Idex/Types/S_ContraintesAxes` _value)))) (`.limiteAmplitude_6_B89E3C1940B78CDC8FB9638773D52084` (break `/Game/Idex/Types/S_Physique` (`.y_7_E9BF3B1347812DAA96BB5DA2DA3EA730` (break `/Game/Idex/Types/S_ContraintesAxes` _value)))) (`/Game/Idex/Classes/Abstraites/BPFL_Contrainte.etatPhysiqueAngulaire` (break `/Game/Idex/Types/S_Physique` (break `/Game/Idex/Types/S_ContraintesAxes` _value))) (`.limiteAmplitude_6_B89E3C1940B78CDC8FB9638773D52084` (break `/Game/Idex/Types/S_Physique` (break `/Game/Idex/Types/S_ContraintesAxes` _value))))
      (set `local.cadreRotation` (`KismetMathLibrary.MakeRotator` (`.limiteCentre_7_B143762145DDCD4F0453E6A849C59040` (break `/Game/Idex/Types/S_Physique` (break `/Game/Idex/Types/S_ContraintesAxes` _value))) (`.limiteCentre_7_B143762145DDCD4F0453E6A849C59040` (break `/Game/Idex/Types/S_Physique` (`.y_7_E9BF3B1347812DAA96BB5DA2DA3EA730` (break `/Game/Idex/Types/S_ContraintesAxes` _value)))) (`.limiteCentre_7_B143762145DDCD4F0453E6A849C59040` (break `/Game/Idex/Types/S_Physique` (`.z_9_09505AF14F2C322AC4DA548E40D9C07C` (break `/Game/Idex/Types/S_ContraintesAxes` _value)))))))
    (:`then_3`
      ; S'il y a au moins une contrainte limitée
      (bind _etat (`/Game/Idex/Classes/Abstraites/BPML_Contrainte.pourChaqueEtat` (`local.contraintes`))
        (:`fin`
          (if (`|EnumEquality` (break `/Game/Idex/Types/S_Physique` (`.physique_9_6356AE914CF5DA94CF165AA84A44D1BA` (break `/Game/Idex/Types/S_Contrainte` _etat))) "NewEnumerator1")
            ;[1 0.15 0.15 0.5] Erreur : l'amplitude limite s'applique autour du point de départ (le transform donné est incorrect)
            (`PhysicsConstraintComponent.SetConstraintReferenceFrame` (`local.composant`) "Frame2" (`/Game/Idex/Classes/Abstraites/BPFL_Transformation.additionner` (`/Game/Idex/Classes/Abstraites/BPFL_Transformation.additionner` (`/Game/Idex/Classes/Abstraites/BPFL_Transformation.soustraire` _returnvalue (`SceneComponent.K2_GetComponentToWorld` (`local.pieceB`))) _returnvalue_2) (`KismetMathLibrary.MakeTransform` (`KismetMathLibrary.TransformDirection` _returnvalue_2 (`local.cadreTranslation`)) (`KismetMathLibrary.TransformRotation` _returnvalue_2 (`local.cadreRotation`)))))))))))

(fn `rafraichir`
  (locals (pieceA :type "StaticMeshComponent Object Reference") (pieceB :type "StaticMeshComponent Object Reference"))
  (bind _piecea (`local.pieceA`))
  ; On réajuste la position et l'orientation de la contrainte pour correspondre à l'état actuel de chaque pièce
  (bind (_keypin _valuepin) (`|MapForEach` (`self.adjacences`))
    (:`then`
      (set `local.pieceA` _keypin)
      (bind (_keypin_2 _valuepin_2) (`|MapForEach` (break `/Game/Idex/Types/S_PiecesLiees` _valuepin))
        (:`then`
          (if (not (== _keypin_2 _piecea))
            (set `local.pieceB` _piecea))
          (`PhysicsConstraintComponent.SetConstrainedComponents` _valuepin_2 (`local.pieceA`) "None" (`local.pieceB`) "None"))))))

(fn `UserConstructionScript`)